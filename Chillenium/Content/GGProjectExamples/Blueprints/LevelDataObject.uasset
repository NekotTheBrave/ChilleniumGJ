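; LevelDataObject holds per-level lists of collected pickups and destroyed enemies and removes those actors from the world when that data is loaded.
; LoadCollectedPickups loops over CollectedPickups and destroys each valid actor reference.
; LoadDestroyedEnemies does the same for DestroyedEnemies, but nests the destroy loop inside an outer loop that prints each enemy's name, so the full destroy pass repeats per entry.
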(fn `LoadCollectedPickups`
  (if (> (`KismetArrayLibrary.Array_Length` (`self.CollectedPickups`)) 0)
    (for _array_element (`self.CollectedPickups`)
      (`/Engine/EditorBlueprintResources/StandardMacros.IsValid` _array_element
        (:`Is Valid`
          (`Actor.K2_DestroyActor` _array_element))))))

(fn `LoadDestroyedEnemies`
  (bind _destroyedenemies (`self.DestroyedEnemies`))
  (for _array_element _destroyedenemies
    (`KismetSystemLibrary.PrintString` null (`KismetSystemLibrary.GetDisplayName` _array_element))
    (if (> (`KismetArrayLibrary.Array_Length` _destroyedenemies) 0)
      (for _array_element_2 (`self.DestroyedEnemies`)
        (`/Engine/EditorBlueprintResources/StandardMacros.IsValid` _array_element_2
          (:`Is Valid`
            (`Actor.K2_DestroyActor` _array_element_2)))))))