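; Falling-block trap that arms shortly after anything overlaps its trigger Box, then drops nine cubes at random.
; Once triggered, delayed Tick rolls per cube enable physics on matches and destroy each 10 seconds later.
; Cube9 never drops, as RandomInteger(9) cannot return 9.
; Overlapping Box1–Box9 damages GothGirlCharacter through DamagePlayer, far more heavily when she is running.
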(event `DamagePlayer`
  (params (OtherActor :type "Actor Object Reference"))
  (bind _asgoth_girl_character (cast `/Game/GGProjectExamples/GothGirlCharacter/GothGirlCharacter` OtherActor))
  (if (`/Game/GGProjectExamples/GothGirlCharacter/GothGirlCharacter.IsRunning` _asgoth_girl_character)
    (set `/Game/GGProjectExamples/GothGirlCharacter/GothGirlCharacter.CurrentHealth` (- (`/Game/GGProjectExamples/GothGirlCharacter/GothGirlCharacter.CurrentHealth` _asgoth_girl_character) 100.0) _asgoth_girl_character)
    (else
      (set `/Game/GGProjectExamples/GothGirlCharacter/GothGirlCharacter.CurrentHealth` (- (`/Game/GGProjectExamples/GothGirlCharacter/GothGirlCharacter.CurrentHealth` _asgoth_girl_character) 1.0) _asgoth_girl_character))))

(event `self.Box.OnComponentBeginOverlap`
  (params (OverlappedComponent :type "PrimitiveComponent Object Reference") (OtherActor :type "Actor Object Reference") (OtherComp :type "PrimitiveComponent Object Reference") (OtherBodyIndex :type Integer) (bFromSweep :type Boolean) (SweepResult :type "HitResult Structure (by ref)"))
  (`KismetSystemLibrary.Delay` 0.2)
  (set `self.Triggered` true))

(event `self.ReceiveTick`
  (params (DeltaSeconds :type "Float (single-precision)"))
  (bind _returnvalue (`KismetMathLibrary.RandomInteger` 9))
  (if (`self.Triggered`)
    (`KismetSystemLibrary.Delay` 0.1)
    (`|ExecutionSequence`
      (:`then_0`
        (if (== _returnvalue 1)
          (bind _cube1 (`self.Cube1`)
            (:`then`
              (`PrimitiveComponent.SetSimulatePhysics` _cube1 true)
              (`KismetSystemLibrary.Delay` 10.0)
              (`ActorComponent.K2_DestroyComponent` _cube1))
            (:`else`))))
      (:`then_1`
        (if (== _returnvalue 2)
          (bind _cube2 (`self.Cube2`)
            (:`then`
              (`PrimitiveComponent.SetSimulatePhysics` _cube2 true)
              (`KismetSystemLibrary.Delay` 10.0)
              (`ActorComponent.K2_DestroyComponent` _cube2))
            (:`else`))))
      (:`then_2`
        (if (== _returnvalue 3)
          (bind _cube3 (`self.Cube3`)
            (:`then`
              (`PrimitiveComponent.SetSimulatePhysics` _cube3 true)
              (`KismetSystemLibrary.Delay` 10.0)
              (`ActorComponent.K2_DestroyComponent` _cube3))
            (:`else`))))
      (:`then_3`
        (if (== _returnvalue 4)
          (bind _cube4 (`self.Cube4`)
            (:`then`
              (`PrimitiveComponent.SetSimulatePhysics` _cube4 true)
              (`KismetSystemLibrary.Delay` 10.0)
              (`ActorComponent.K2_DestroyComponent` _cube4))
            (:`else`))))
      (:`then_4`
        (if (== _returnvalue 5)
          (bind _cube5 (`self.Cube5`)
            (:`then`
              (`PrimitiveComponent.SetSimulatePhysics` _cube5 true)
              (`KismetSystemLibrary.Delay` 10.0)
              (`ActorComponent.K2_DestroyComponent` _cube5))
            (:`else`))))
      (:`then_5`
        (if (== _returnvalue 6)
          (bind _cube6 (`self.Cube6`)
            (:`then`
              (`PrimitiveComponent.SetSimulatePhysics` _cube6 true)
              (`KismetSystemLibrary.Delay` 10.0)
              (`ActorComponent.K2_DestroyComponent` _cube6))
            (:`else`))))
      (:`then_6`
        (if (== _returnvalue 7)
          (bind _cube7 (`self.Cube7`)
            (:`then`
              (`PrimitiveComponent.SetSimulatePhysics` _cube7 true)
              (`KismetSystemLibrary.Delay` 10.0)
              (`ActorComponent.K2_DestroyComponent` _cube7))
            (:`else`))))
      (:`then_7`
        (if (== _returnvalue 8)
          (bind _cube8 (`self.Cube8`)
            (:`then`
              (`PrimitiveComponent.SetSimulatePhysics` _cube8 true)
              (`KismetSystemLibrary.Delay` 10.0)
              (`ActorComponent.K2_DestroyComponent` _cube8))
            (:`else`))))
      (:`then_8`
        (if (== _returnvalue 9)
          (bind _cube9 (`self.Cube9`)
            (:`then`
              (`PrimitiveComponent.SetSimulatePhysics` _cube9 true)
              (`KismetSystemLibrary.Delay` 10.0)
              (`ActorComponent.K2_DestroyComponent` _cube9))
            (:`else`)))))))

(event `self.Box1.OnComponentBeginOverlap`
  (params (OverlappedComponent :type "PrimitiveComponent Object Reference") (OtherActor :type "Actor Object Reference") (OtherComp :type "PrimitiveComponent Object Reference") (OtherBodyIndex :type Integer) (bFromSweep :type Boolean) (SweepResult :type "HitResult Structure (by ref)"))
  (`self.DamagePlayer` OtherActor))

(event `self.Box2.OnComponentBeginOverlap`
  (params (OverlappedComponent :type "PrimitiveComponent Object Reference") (OtherActor :type "Actor Object Reference") (OtherComp :type "PrimitiveComponent Object Reference") (OtherBodyIndex :type Integer) (bFromSweep :type Boolean) (SweepResult :type "HitResult Structure (by ref)"))
  (`self.DamagePlayer` OtherActor))

(event `self.Box3.OnComponentBeginOverlap`
  (params (OverlappedComponent :type "PrimitiveComponent Object Reference") (OtherActor :type "Actor Object Reference") (OtherComp :type "PrimitiveComponent Object Reference") (OtherBodyIndex :type Integer) (bFromSweep :type Boolean) (SweepResult :type "HitResult Structure (by ref)"))
  (`self.DamagePlayer` OtherActor))

(event `self.Box4.OnComponentBeginOverlap`
  (params (OverlappedComponent :type "PrimitiveComponent Object Reference") (OtherActor :type "Actor Object Reference") (OtherComp :type "PrimitiveComponent Object Reference") (OtherBodyIndex :type Integer) (bFromSweep :type Boolean) (SweepResult :type "HitResult Structure (by ref)"))
  (`self.DamagePlayer` OtherActor))

(event `self.Box5.OnComponentBeginOverlap`
  (params (OverlappedComponent :type "PrimitiveComponent Object Reference") (OtherActor :type "Actor Object Reference") (OtherComp :type "PrimitiveComponent Object Reference") (OtherBodyIndex :type Integer) (bFromSweep :type Boolean) (SweepResult :type "HitResult Structure (by ref)"))
  (`self.DamagePlayer` OtherActor))

(event `self.Box6.OnComponentBeginOverlap`
  (params (OverlappedComponent :type "PrimitiveComponent Object Reference") (OtherActor :type "Actor Object Reference") (OtherComp :type "PrimitiveComponent Object Reference") (OtherBodyIndex :type Integer) (bFromSweep :type Boolean) (SweepResult :type "HitResult Structure (by ref)"))
  (`self.DamagePlayer` OtherActor))

(event `self.Box7.OnComponentBeginOverlap`
  (params (OverlappedComponent :type "PrimitiveComponent Object Reference") (OtherActor :type "Actor Object Reference") (OtherComp :type "PrimitiveComponent Object Reference") (OtherBodyIndex :type Integer) (bFromSweep :type Boolean) (SweepResult :type "HitResult Structure (by ref)"))
  (`self.DamagePlayer` OtherActor))

(event `self.Box8.OnComponentBeginOverlap`
  (params (OverlappedComponent :type "PrimitiveComponent Object Reference") (OtherActor :type "Actor Object Reference") (OtherComp :type "PrimitiveComponent Object Reference") (OtherBodyIndex :type Integer) (bFromSweep :type Boolean) (SweepResult :type "HitResult Structure (by ref)"))
  (`self.DamagePlayer` OtherActor))

(event `self.Box9.OnComponentBeginOverlap`
  (params (OverlappedComponent :type "PrimitiveComponent Object Reference") (OtherActor :type "Actor Object Reference") (OtherComp :type "PrimitiveComponent Object Reference") (OtherBodyIndex :type Integer) (bFromSweep :type Boolean) (SweepResult :type "HitResult Structure (by ref)"))
  (`self.DamagePlayer` OtherActor))

(fn `UserConstructionScript`)