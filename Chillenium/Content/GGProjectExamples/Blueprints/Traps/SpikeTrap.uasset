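; Spike trap that raises its spikes after a short delay when something overlaps its trigger box, hurting the GothGirlCharacter.
; Tick interpolates Cube1 upward, holds it during a cooldown, then retracts it more slowly to its saved starting position.
; Trigger, cooldown and retract flags stop the trap from re-firing mid-cycle.
; Overlapping any spike or cone subtracts health from the character, far more if they are running.
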(event `DamagePlayer`
  (params (OtherActor :type "Actor Object Reference"))
  (bind _asgoth_girl_character (cast `/Game/GGProjectExamples/GothGirlCharacter/GothGirlCharacter` OtherActor))
  (if (`/Game/GGProjectExamples/GothGirlCharacter/GothGirlCharacter.IsRunning` _asgoth_girl_character)
    (set `/Game/GGProjectExamples/GothGirlCharacter/GothGirlCharacter.CurrentHealth` (- (`/Game/GGProjectExamples/GothGirlCharacter/GothGirlCharacter.CurrentHealth` _asgoth_girl_character) 100.0) _asgoth_girl_character)
    (else
      (set `/Game/GGProjectExamples/GothGirlCharacter/GothGirlCharacter.CurrentHealth` (- (`/Game/GGProjectExamples/GothGirlCharacter/GothGirlCharacter.CurrentHealth` _asgoth_girl_character) 1.0) _asgoth_girl_character))))

(event `self.Box.OnComponentBeginOverlap`
  (params (OverlappedComponent :type "PrimitiveComponent Object Reference") (OtherActor :type "Actor Object Reference") (OtherComp :type "PrimitiveComponent Object Reference") (OtherBodyIndex :type Integer) (bFromSweep :type Boolean) (SweepResult :type "HitResult Structure (by ref)"))
  (`KismetSystemLibrary.Delay` 0.2)
  (if (and (not (`self.Cooldown`)) (not (`self.Triggered`)) (not (`self.Retracting`)))
    (set `self.Current Location` (`SceneComponent.K2_GetComponentLocation` (`self.Cube1`)))
    (set `self.Triggered` true)))

(event `self.ReceiveTick`
  (params (DeltaSeconds :type "Float (single-precision)"))
  (bind _cube1 (`self.Cube1`))
  (bind _current_location (`self.Current Location`))
  (bind _returnvalue (`SceneComponent.K2_GetComponentRotation` _cube1))
  (bind _returnvalue_2 (`SceneComponent.K2_GetComponentLocation` _cube1))
  (bind _returnvalue_3 (`SceneComponent.K2_GetComponentRotation` _cube1))
  (bind _returnvalue_4 (+ _current_location (0.0 0.0 120.0)))
  (bind _returnvalue_location (`KismetMathLibrary.BreakTransform` (`KismetMathLibrary.TInterpTo` (`KismetMathLibrary.MakeTransform` _returnvalue_2 _returnvalue_3) (`KismetMathLibrary.MakeTransform` _current_location _returnvalue_3) (`GameplayStatics.GetWorldDeltaSeconds`) 4.0)))
  (bind _returnvalue_location_2 (`KismetMathLibrary.BreakTransform` (`KismetMathLibrary.TInterpTo` (`KismetMathLibrary.MakeTransform` _returnvalue_2 _returnvalue) (`KismetMathLibrary.MakeTransform` _returnvalue_4 _returnvalue) (`GameplayStatics.GetWorldDeltaSeconds`) 10.0)))
  (if (`self.Retracting`)
    (if (== _returnvalue_2 _current_location :`ErrorTolerance` 2.0)
      (set `self.Retracting` false)
      (set `self.Cooldown` false)
      (else
        (`SceneComponent.K2_SetWorldLocation` _cube1 _returnvalue_location false false)))
    (elif (`self.Triggered`)
      (if (== _returnvalue_2 _returnvalue_4 :`ErrorTolerance` 2.0)
        (set `self.Triggered` false)
        (set `self.Cooldown` true)
        (`KismetSystemLibrary.Delay` 5.0)
        (set `self.Retracting` true)
        (else
          (`SceneComponent.K2_SetWorldLocation` _cube1 _returnvalue_location_2 false false))))))

(event `self.Spike 2.OnComponentBeginOverlap`
  (params (OverlappedComponent :type "PrimitiveComponent Object Reference") (OtherActor :type "Actor Object Reference") (OtherComp :type "PrimitiveComponent Object Reference") (OtherBodyIndex :type Integer) (bFromSweep :type Boolean) (SweepResult :type "HitResult Structure (by ref)"))
  (`self.DamagePlayer` OtherActor))

(event `self.Spike 3.OnComponentBeginOverlap`
  (params (OverlappedComponent :type "PrimitiveComponent Object Reference") (OtherActor :type "Actor Object Reference") (OtherComp :type "PrimitiveComponent Object Reference") (OtherBodyIndex :type Integer) (bFromSweep :type Boolean) (SweepResult :type "HitResult Structure (by ref)"))
  (`self.DamagePlayer` OtherActor))

(event `self.Spike 4.OnComponentBeginOverlap`
  (params (OverlappedComponent :type "PrimitiveComponent Object Reference") (OtherActor :type "Actor Object Reference") (OtherComp :type "PrimitiveComponent Object Reference") (OtherBodyIndex :type Integer) (bFromSweep :type Boolean) (SweepResult :type "HitResult Structure (by ref)"))
  (`self.DamagePlayer` OtherActor))

(event `self.Spike 5.OnComponentBeginOverlap`
  (params (OverlappedComponent :type "PrimitiveComponent Object Reference") (OtherActor :type "Actor Object Reference") (OtherComp :type "PrimitiveComponent Object Reference") (OtherBodyIndex :type Integer) (bFromSweep :type Boolean) (SweepResult :type "HitResult Structure (by ref)"))
  (`self.DamagePlayer` OtherActor))

(event `self.Spike 1.OnComponentBeginOverlap`
  (params (OverlappedComponent :type "PrimitiveComponent Object Reference") (OtherActor :type "Actor Object Reference") (OtherComp :type "PrimitiveComponent Object Reference") (OtherBodyIndex :type Integer) (bFromSweep :type Boolean) (SweepResult :type "HitResult Structure (by ref)"))
  (`self.DamagePlayer` OtherActor))

(event `self.Cone.OnComponentBeginOverlap`
  (params (OverlappedComponent :type "PrimitiveComponent Object Reference") (OtherActor :type "Actor Object Reference") (OtherComp :type "PrimitiveComponent Object Reference") (OtherBodyIndex :type Integer) (bFromSweep :type Boolean) (SweepResult :type "HitResult Structure (by ref)"))
  (`self.DamagePlayer` OtherActor))

(event `self.Cone1.OnComponentBeginOverlap`
  (params (OverlappedComponent :type "PrimitiveComponent Object Reference") (OtherActor :type "Actor Object Reference") (OtherComp :type "PrimitiveComponent Object Reference") (OtherBodyIndex :type Integer) (bFromSweep :type Boolean) (SweepResult :type "HitResult Structure (by ref)"))
  (`self.DamagePlayer` OtherActor))

(event `self.Cone2.OnComponentBeginOverlap`
  (params (OverlappedComponent :type "PrimitiveComponent Object Reference") (OtherActor :type "Actor Object Reference") (OtherComp :type "PrimitiveComponent Object Reference") (OtherBodyIndex :type Integer) (bFromSweep :type Boolean) (SweepResult :type "HitResult Structure (by ref)"))
  (`self.DamagePlayer` OtherActor))

(event `self.Cone3.OnComponentBeginOverlap`
  (params (OverlappedComponent :type "PrimitiveComponent Object Reference") (OtherActor :type "Actor Object Reference") (OtherComp :type "PrimitiveComponent Object Reference") (OtherBodyIndex :type Integer) (bFromSweep :type Boolean) (SweepResult :type "HitResult Structure (by ref)"))
  (`self.DamagePlayer` OtherActor))

(fn `UserConstructionScript`)