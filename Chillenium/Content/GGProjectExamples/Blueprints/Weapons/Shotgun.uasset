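; Shotgun weapon item whose UseItem override equips it on the player's GothGirlCharacter, provided the character has the shotgun.
; Depending on character state, it first triggers sheathing, then attaches the existing shotgun, or a newly spawned one with collision disabled, to the right-hand socket.
; It clears equipped flags on pistols, Uzis and Magnums through nested validity checks.
; Final weapon-state and animation updates run only when both pistol references are valid.
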(fn `UseItem`
  (returns (Success :type Boolean))
  (bind _success (`parent.UseItem`))
  (bind _asgoth_girl_character (cast `/Game/GGProjectExamples/GothGirlCharacter/GothGirlCharacter` (`GameplayStatics.GetPlayerCharacter` 0)))
  (if (`/Game/GGProjectExamples/GothGirlCharacter/GothGirlCharacter.HasShotgun` _asgoth_girl_character)
    (if (`|EnumEquality` (`/Game/GGProjectExamples/GothGirlCharacter/GothGirlCharacter.CurrentState` _asgoth_girl_character) "NewEnumerator0")
      (bind _output_get (set `/Game/GGProjectExamples/GothGirlCharacter/GothGirlCharacter.DrawAfterEquip` true _asgoth_girl_character))
      (message `/Game/GGProjectExamples/Blueprints/ArmedWeapon.Sheathed` _asgoth_girl_character)
      (set `/Game/GGProjectExamples/GothGirlCharacter/GothGirlCharacter.WeaponEquippedState` "NewEnumerator3" _asgoth_girl_character)
      (message `/Game/GGProjectExamples/Blueprints/ArmedWeapon.Aiming` (`SkeletalMeshComponent.GetAnimInstance` (`Character.Mesh` _asgoth_girl_character)) false false false))
    (if (`KismetSystemLibrary.IsValid` (`/Game/GGProjectExamples/GothGirlCharacter/GothGirlCharacter.ShotgunEquipped` _asgoth_girl_character))
      (bind _shotgunequipped (`/Game/GGProjectExamples/GothGirlCharacter/GothGirlCharacter.ShotgunEquipped` _asgoth_girl_character)
        (:`then`
          (bind _mesh (`Character.Mesh` _asgoth_girl_character))
          (`self.K2_AttachToComponent` _shotgunequipped _mesh "RightHandShotgun" "SnapToTarget" "SnapToTarget" "SnapToTarget" true))
        (:`else`))
      (else
        (bind _returnvalue (`|SpawnActorFromClass` "Shotgun_C" (`KismetMathLibrary.MakeTransform` (0.0 0.0 0.0)) "Undefined" "OverrideRootScale" null null))
        (bind _output_get_2 (set `/Game/GGProjectExamples/GothGirlCharacter/GothGirlCharacter.ShotgunEquipped` _returnvalue _asgoth_girl_character))
        (`PrimitiveComponent.SetCollisionEnabled` (`/Game/GGProjectExamples/Blueprints/Pickups/Item.ItemInteractCollision` _output_get_2) "NoCollision")
        (`PrimitiveComponent.SetCollisionEnabled` (`/Game/GGProjectExamples/Blueprints/Pickups/Item.ItemRadius` _output_get_2) "NoCollision")
        (`PrimitiveComponent.SetCollisionEnabled` (`/Game/GGProjectExamples/Blueprints/Pickups/Item.BaseMesh` _output_get_2) "NoCollision")
        (`self.K2_AttachToComponent` _returnvalue _mesh "RightHandShotgun" "SnapToTarget" "SnapToTarget" "SnapToTarget" true)
        (`self.K2_AttachToComponent` _output_get_2 _mesh "RightHandShotgun" "SnapToTarget" "SnapToTarget" "SnapToTarget" true)))
    (set `self.IsEquipped` true)
    (bind _pistol1eqipped (`/Game/GGProjectExamples/GothGirlCharacter/GothGirlCharacter.Pistol1Eqipped` _asgoth_girl_character)
      (:`then`
        (set `/Game/GGProjectExamples/Blueprints/Pickups/Item.IsEquipped` false _pistol1eqipped)
        (bind _pistol2equipped (`/Game/GGProjectExamples/GothGirlCharacter/GothGirlCharacter.Pistol2Equipped` _asgoth_girl_character)
          (:`then`
            (set `/Game/GGProjectExamples/Blueprints/Pickups/Item.IsEquipped` false _pistol2equipped)
            (bind _uzi1equipped (`/Game/GGProjectExamples/GothGirlCharacter/GothGirlCharacter.Uzi1Equipped` _asgoth_girl_character)
              (:`then`
                (set `/Game/GGProjectExamples/Blueprints/Pickups/Item.IsEquipped` false _uzi1equipped)
                (bind _uzi2equipped (`/Game/GGProjectExamples/GothGirlCharacter/GothGirlCharacter.Uzi2Equipped` _asgoth_girl_character)
                  (:`then`
                    (set `/Game/GGProjectExamples/Blueprints/Pickups/Item.IsEquipped` false _uzi2equipped))
                  (:`else`
                    _)))
              (:`else`
                _))
            (bind _magnum1equipped (`/Game/GGProjectExamples/GothGirlCharacter/GothGirlCharacter.Magnum1Equipped` _asgoth_girl_character)
              (:`then`
                (set `/Game/GGProjectExamples/Blueprints/Pickups/Item.IsEquipped` false _magnum1equipped)
                (bind _magnum2equipped (`/Game/GGProjectExamples/GothGirlCharacter/GothGirlCharacter.Magnum2Equipped` _asgoth_girl_character)
                  (:`then`
                    (set `/Game/GGProjectExamples/Blueprints/Pickups/Item.IsEquipped` false _magnum2equipped))
                  (:`else`
                    _)))
              (:`else`
                _))
            (if _output_get
              (set `/Game/GGProjectExamples/GothGirlCharacter/GothGirlCharacter.WeaponEquippedState` "NewEnumerator1" _asgoth_girl_character)
              (else
                (set `/Game/GGProjectExamples/GothGirlCharacter/GothGirlCharacter.WeaponEquippedState` "NewEnumerator1" _asgoth_girl_character)
                (set `/Game/GGProjectExamples/GothGirlCharacter/GothGirlCharacter.CurrentState` "NewEnumerator0" _asgoth_girl_character)
                (bind _returnvalue_2 (`SkeletalMeshComponent.GetAnimInstance` _mesh))
                (message `/Game/GGProjectExamples/Blueprints/ArmedWeapon.Drawn` _returnvalue_2)
                (message `/Game/GGProjectExamples/Blueprints/ArmedWeapon.Aiming` _returnvalue_2 false true false)))
            (return _success))
          (:`else`)))
      (:`else`))))

(fn `UserConstructionScript`
  (`parent.UserConstructionScript`))