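; Dual pistols weapon item that equips a pistol in each hand of the GothGirlCharacter when used.
; UseItem extends the parent, spawning two Pistols actors if none exist, snapping them to hand sockets and disabling their collision.
; It flags any shotgun as unequipped, destroys equipped Uzis and Magnums, then updates the character's weapon state and messages its AnimInstance to handle drawn and aiming poses.
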(fn `UseItem`
  (returns (Success :type Boolean))
  (bind _success (`parent.UseItem`))
  (bind _asgoth_girl_character (cast `/Game/GGProjectExamples/GothGirlCharacter/GothGirlCharacter` (`GameplayStatics.GetPlayerCharacter` 0)))
  (if (`|EnumEquality` (`/Game/GGProjectExamples/GothGirlCharacter/GothGirlCharacter.CurrentState` _asgoth_girl_character) "NewEnumerator0")
    (bind _output_get (set `/Game/GGProjectExamples/GothGirlCharacter/GothGirlCharacter.DrawAfterEquip` true _asgoth_girl_character))
    (message `/Game/GGProjectExamples/Blueprints/ArmedWeapon.Sheathed` _asgoth_girl_character)
    (set `/Game/GGProjectExamples/GothGirlCharacter/GothGirlCharacter.WeaponEquippedState` "NewEnumerator2" _asgoth_girl_character)
    (message `/Game/GGProjectExamples/Blueprints/ArmedWeapon.Aiming` (`SkeletalMeshComponent.GetAnimInstance` (`Character.Mesh` _asgoth_girl_character)) false false false))
  (if (not (`KismetSystemLibrary.IsValid` (`/Game/GGProjectExamples/GothGirlCharacter/GothGirlCharacter.Pistol1Eqipped` _asgoth_girl_character)))
    (bind _returnvalue (`|SpawnActorFromClass` "Pistols_C" (`KismetMathLibrary.MakeTransform` (0.0 0.0 0.0)) "Undefined" "OverrideRootScale" null null))
    (bind _output_get_2 (set `/Game/GGProjectExamples/GothGirlCharacter/GothGirlCharacter.Pistol1Eqipped` _returnvalue _asgoth_girl_character))
    (bind _returnvalue_2 (`|SpawnActorFromClass` "Pistols_C" (`KismetMathLibrary.MakeTransform` (0.0 0.0 0.0)) "Undefined" "OverrideRootScale" null null))
    (bind _output_get_3 (set `/Game/GGProjectExamples/GothGirlCharacter/GothGirlCharacter.Pistol2Equipped` _returnvalue_2 _asgoth_girl_character)))
  (bind _pistol1eqipped (`/Game/GGProjectExamples/GothGirlCharacter/GothGirlCharacter.Pistol1Eqipped` _asgoth_girl_character))
  (bind _mesh (`Character.Mesh` _asgoth_girl_character))
  (`self.K2_AttachToComponent` _pistol1eqipped _mesh "RightHandPistol" "SnapToTarget" "SnapToTarget" "SnapToTarget" true)
  (`self.K2_AttachToComponent` _output_get_2 _mesh "RightHandPistol" "SnapToTarget" "SnapToTarget" "SnapToTarget" true)
  (bind _pistol2equipped (`/Game/GGProjectExamples/GothGirlCharacter/GothGirlCharacter.Pistol2Equipped` _asgoth_girl_character))
  (`self.K2_AttachToComponent` _pistol2equipped _mesh "LeftHandPistol" "SnapToTarget" "SnapToTarget" "SnapToTarget" true)
  (`self.K2_AttachToComponent` _output_get_3 _mesh "LeftHandPistol" "SnapToTarget" "SnapToTarget" "SnapToTarget" true)
  (`PrimitiveComponent.SetCollisionEnabled` (`/Game/GGProjectExamples/Blueprints/Pickups/Item.ItemInteractCollision` _output_get_3) "NoCollision")
  (`PrimitiveComponent.SetCollisionEnabled` (`/Game/GGProjectExamples/Blueprints/Pickups/Item.ItemRadius` _output_get_3) "NoCollision")
  (`PrimitiveComponent.SetCollisionEnabled` (`/Game/GGProjectExamples/Blueprints/Pickups/Item.BaseMesh` _output_get_3) "NoCollision")
  (`PrimitiveComponent.SetCollisionEnabled` (`/Game/GGProjectExamples/Blueprints/Pickups/Item.ItemInteractCollision` _output_get_2) "NoCollision")
  (`PrimitiveComponent.SetCollisionEnabled` (`/Game/GGProjectExamples/Blueprints/Pickups/Item.ItemRadius` _output_get_2) "NoCollision")
  (`PrimitiveComponent.SetCollisionEnabled` (`/Game/GGProjectExamples/Blueprints/Pickups/Item.BaseMesh` _output_get_2) "NoCollision")
  (bind _shotgunequipped (`/Game/GGProjectExamples/GothGirlCharacter/GothGirlCharacter.ShotgunEquipped` _asgoth_girl_character))
  (`/Engine/EditorBlueprintResources/StandardMacros.IsValid` _shotgunequipped
    (:`Is Valid`
      (set `/Game/GGProjectExamples/Blueprints/Pickups/Item.IsEquipped` false _shotgunequipped))
    (:`Is Not Valid`
      _))
  (set `/Game/GGProjectExamples/Blueprints/Pickups/Item.IsEquipped` true _pistol2equipped)
  (set `/Game/GGProjectExamples/Blueprints/Pickups/Item.IsEquipped` true _pistol1eqipped)
  (bind _uzi1equipped (`/Game/GGProjectExamples/GothGirlCharacter/GothGirlCharacter.Uzi1Equipped` _asgoth_girl_character)
    (:`then`
      (set `/Game/GGProjectExamples/Blueprints/Pickups/Item.IsEquipped` false _uzi1equipped)
      (`self.K2_DestroyActor` _uzi1equipped)
      (bind _uzi2equipped (`/Game/GGProjectExamples/GothGirlCharacter/GothGirlCharacter.Uzi2Equipped` _asgoth_girl_character)
        (:`then`
          (set `/Game/GGProjectExamples/Blueprints/Pickups/Item.IsEquipped` false _uzi2equipped)
          (`self.K2_DestroyActor` _uzi2equipped))
        (:`else`
          _)))
    (:`else`
      _))
  (bind _magnum1equipped (`/Game/GGProjectExamples/GothGirlCharacter/GothGirlCharacter.Magnum1Equipped` _asgoth_girl_character)
    (:`then`
      (set `/Game/GGProjectExamples/Blueprints/Pickups/Item.IsEquipped` false _magnum1equipped)
      (`self.K2_DestroyActor` _magnum1equipped)
      (bind _magnum2equipped (`/Game/GGProjectExamples/GothGirlCharacter/GothGirlCharacter.Magnum2Equipped` _asgoth_girl_character)
        (:`then`
          (set `/Game/GGProjectExamples/Blueprints/Pickups/Item.IsEquipped` false _magnum2equipped)
          (`self.K2_DestroyActor` _magnum2equipped))
        (:`else`
          _)))
    (:`else`
      _))
  (if _output_get
    (set `/Game/GGProjectExamples/GothGirlCharacter/GothGirlCharacter.WeaponEquippedState` "NewEnumerator0" _asgoth_girl_character)
    (`KismetSystemLibrary.PrintString` "Alreday equipped")
    (else
      (set `/Game/GGProjectExamples/GothGirlCharacter/GothGirlCharacter.WeaponEquippedState` "NewEnumerator0" _asgoth_girl_character)
      (set `/Game/GGProjectExamples/GothGirlCharacter/GothGirlCharacter.CurrentState` "NewEnumerator0" _asgoth_girl_character)
      (bind _returnvalue_3 (`SkeletalMeshComponent.GetAnimInstance` _mesh))
      (message `/Game/GGProjectExamples/Blueprints/ArmedWeapon.Drawn` _returnvalue_3)))
  (message `/Game/GGProjectExamples/Blueprints/ArmedWeapon.Aiming` _returnvalue_3 false true false)
  (return _success))

(fn `UserConstructionScript`
  (`parent.UserConstructionScript`))