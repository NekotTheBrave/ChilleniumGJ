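; Lever pickup that the GothGirlCharacter pulls to sink a linked InteractedObject, such as a barrier, downward by most of its height.
; Interact plays character and lever montages while Tick interpolates the character into position and rotation beside the lever.
; After timed delays it calls TrackPoint on the Camera and starts the drop.
; Tick then lowers the object using its bounds, and flags keep the drop one-shot.
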(event `self.ReceiveTick`
  (params (DeltaSeconds :type "Float (single-precision)"))
  (bind (_returnvalue_roll _returnvalue_pitch _returnvalue_yaw) (`KismetMathLibrary.BreakRotator` (`self.K2_GetActorRotation`)))
  (bind _returnvalue_x (`KismetMathLibrary.BreakVector` (`self.GetActorForwardVector`)))
  (bind _interactedobject (`self.InteractedObject`))
  (bind (_returnvalue_x_2 _returnvalue_y _returnvalue_z) (`KismetMathLibrary.BreakVector` (`self.K2_GetActorLocation` _interactedobject)))
  (bind (_returnvalue_x_3 _returnvalue_y_2 _returnvalue_z_2) (`KismetMathLibrary.BreakVector` (`self.K2_GetActorLocation` (`self.InteractedObject`))))
  (bind (_returnvalue_x_4 _returnvalue_y_3) (`KismetMathLibrary.BreakVector` (- (`self.K2_GetActorLocation`) (`KismetMathLibrary.MakeVector` 0.0 (* -100.0 _returnvalue_x)))))
  (if (`self.Translating`)
    (`self.K2_SetActorRotation` (stale `/Game/GGProjectExamples/Blueprints/InteractInterface.Interact` _asgoth_girl_character) (`KismetMathLibrary.RInterpTo` (`self.K2_GetActorRotation` (stale `/Game/GGProjectExamples/Blueprints/InteractInterface.Interact` _asgoth_girl_character)) (`KismetMathLibrary.MakeRotator` _returnvalue_roll _returnvalue_pitch (- _returnvalue_yaw 90.0)) DeltaSeconds 3.0) false)
    (bind (_returnvalue_x_5 _returnvalue_y_4 _returnvalue_z_3) (`KismetMathLibrary.BreakVector` (`self.K2_GetActorLocation` (stale `/Game/GGProjectExamples/Blueprints/InteractInterface.Interact` _asgoth_girl_character))))
    (`self.K2_SetActorLocation` (stale `/Game/GGProjectExamples/Blueprints/InteractInterface.Interact` _asgoth_girl_character) (`KismetMathLibrary.VInterpTo` (`self.K2_GetActorLocation` (stale `/Game/GGProjectExamples/Blueprints/InteractInterface.Interact` _asgoth_girl_character)) (`KismetMathLibrary.MakeVector` _returnvalue_x_4 _returnvalue_y_3 _returnvalue_z_3) DeltaSeconds 3.0) false false)
    (elif (`self.IsTriggered`)
      (`self.K2_SetActorLocation` _interactedobject (`KismetMathLibrary.MakeVector` _returnvalue_x_2 _returnvalue_y (`KismetMathLibrary.FInterpTo` _returnvalue_z (- _returnvalue_z (* (.z (`.BoxExtent` (`self.GetActorBounds` (`self.InteractedObject`) false false))) 2.0)) DeltaSeconds (`self.Speed`))) false false)
      (if (`KismetMathLibrary.NearlyEqual_FloatFloat` _returnvalue_z_2 (- (stale `/Game/GGProjectExamples/Blueprints/InteractInterface.Interact` _output_get) (* (.z (`.BoxExtent` (`self.GetActorBounds` (`self.InteractedObject`) false false))) 1.5)) 1.0)
        (set `self.IsTriggered` false)
        (set `self.HasBeenTriggered` true)))))

(event `/Game/GGProjectExamples/Blueprints/InteractInterface.Interact`
  (params (Interacter :type "Actor Object Reference"))
  (bind (_returnvalue_x _returnvalue_y _returnvalue_z) (`KismetMathLibrary.BreakVector` (`self.K2_GetActorLocation` (`self.InteractedObject`))))
  (bind _asgoth_girl_character (cast `/Game/GGProjectExamples/GothGirlCharacter/GothGirlCharacter` Interacter))
  (`Character.PlayAnimMontage` _asgoth_girl_character "/Game/GGProjectExamples/GothGirlCharacter/GothGirlRootModel/GGLeverPull_Montage.GGLeverPull_Montage" 1.0 "None")
  (set `self.Translating` true)
  (`KismetSystemLibrary.Delay` 0.5)
  (`|PlayMontage` (`self.LeverSM`) "/Game/GGProjectExamples/Blueprints/Pickups/LeverPull_Montage.LeverPull_Montage"
    (:`then`
      (`KismetSystemLibrary.Delay` 1.0)
      (`Character.StopAnimMontage` _asgoth_girl_character "/Game/GGProjectExamples/GothGirlCharacter/GothGirlRootModel/GGLeverPull_Montage.GGLeverPull_Montage")
      (`/Game/GGProjectExamples/Blueprints/DynamicCameraSystem.Track Point` (`self.Camera`))
      (set `self.Translating` false)
      (if (not (or (`self.IsTriggered`) (`self.HasBeenTriggered`)))
        (set `self.IsTriggered` true)
        (bind _output_get (set `self.ZLocation` _returnvalue_z))))))

(fn `UserConstructionScript`
  (`parent.UserConstructionScript`))