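; Key1 is an interactable pickup item that records itself in the level save's collected pickups when a GothGirlCharacter interacts with it.
; If equipped it disables its collision; if pickable it plays a pickup montage, adds itself to the inventory and destroys itself on success.
; Name checks for four weapons set character ownership flags and hide matching child components in 3DMeshCapture, mostly ammo displays.
; UseItem always returns false.
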(event `/Game/GGProjectExamples/Blueprints/InteractInterface.Interact`
  (params (Interacter :type "Actor Object Reference"))
  (bind (_itemstructure_name _itemstructure_description _itemstructure_staticmesh _itemstructure_thumbnail _itemstructure_quantity _itemstructure_damage _itemstructure_class _itemstructure_isconsumable _itemstructure_maxstacksize _itemstructure_isstackable _itemstructure_ispickable) (break `/Game/GGProjectExamples/Blueprints/ItemStructure` (`self.ItemStructure`)))
  (bind (_itemstructure_name_2 _itemstructure_description_2 _itemstructure_staticmesh_2 _itemstructure_thumbnail_2 _itemstructure_quantity_2 _itemstructure_damage_2 _itemstructure_class_2 _itemstructure_isconsumable_2 _itemstructure_maxstacksize_2 _itemstructure_isstackable_2 _itemstructure_ispickable_2 _itemstructure_ammo _itemstructure_isequipped _itemstructure_hasweapon _itemstructure_healingvalue _itemstructure_actor) (break `/Game/GGProjectExamples/Blueprints/ItemStructure` (`self.ItemStructure`)))
  (bind _returnvalue (`KismetTextLibrary.Conv_TextToString` _itemstructure_name))
  (bind _asgoth_girl_character (cast `/Game/GGProjectExamples/GothGirlCharacter/GothGirlCharacter` Interacter))
  (`KismetArrayLibrary.Array_AddUnique` (`/Game/GGProjectExamples/Blueprints/LevelDataObject.CollectedPickups` (`/Game/GGProjectExamples/Blueprints/GothGirlGameInstance.LevelSaveObject` (`/Game/GGProjectExamples/GothGirlCharacter/GothGirlCharacter.GothGirlGameInstance` _asgoth_girl_character))) self)
  (if (`self.IsEquipped`)
    (`PrimitiveComponent.SetCollisionEnabled` (`self.BaseMesh`) "NoCollision")
    (`PrimitiveComponent.SetCollisionEnabled` (`self.ItemRadius`) "NoCollision")
    (`PrimitiveComponent.SetCollisionEnabled` (`self.ItemInteractCollision`) "NoCollision")
    (elif _itemstructure_ispickable
      (bind _asgoth_girl_character_2 (cast `/Game/GGProjectExamples/GothGirlCharacter/GothGirlCharacter` (`GameplayStatics.GetPlayerCharacter` 0)))
      (if (`KismetStringLibrary.EqualEqual_StrStr` _returnvalue "Shotgun")
        (set `/Game/GGProjectExamples/GothGirlCharacter/GothGirlCharacter.HasShotgun` true _asgoth_girl_character_2)
        (bind _outactors (`GameplayStatics.GetAllActorsOfClass` "/Game/GGProjectExamples/UserInterface/RenderTarget/3DMeshCapture.3DMeshCapture_C"))
        (bind _asgoth_girl_character_3 (cast `/Game/GGProjectExamples/GothGirlCharacter/GothGirlCharacter` (`GameplayStatics.GetPlayerCharacter` 0)))
        (for _array_element (`SceneComponent.GetChildrenComponents` (`/Game/GGProjectExamples/UserInterface/RenderTarget/3DMeshCapture.Plane` (`|GetArrayItem` _outactors)) false)
          (for _array_element_2 (`SceneComponent.GetChildrenComponents` _array_element false)
            (if (`KismetStringLibrary.Contains` (`KismetSystemLibrary.GetDisplayName` _array_element_2) "ShotgunAmmo")
              (`SceneComponent.SetVisibility` _array_element_2 false false)
              (set `/Game/GGProjectExamples/Blueprints/InventoryComponent.ShotgunAmmoAdded` false (`/Game/GGProjectExamples/GothGirlCharacter/GothGirlCharacter.InventoryComponent` _asgoth_girl_character_3))
              (else
                (if (`KismetStringLibrary.EqualEqual_StrStr` _returnvalue "Magnums") :!label _label
                  (set `/Game/GGProjectExamples/GothGirlCharacter/GothGirlCharacter.HasMagnums` true _asgoth_girl_character_2)
                  (bind _outactors_2 (`GameplayStatics.GetAllActorsOfClass` "/Game/GGProjectExamples/UserInterface/RenderTarget/3DMeshCapture.3DMeshCapture_C"))
                  (bind _asgoth_girl_character_4 (cast `/Game/GGProjectExamples/GothGirlCharacter/GothGirlCharacter` (`GameplayStatics.GetPlayerCharacter` 0)))
                  (for _array_element_3 (`SceneComponent.GetChildrenComponents` (`/Game/GGProjectExamples/UserInterface/RenderTarget/3DMeshCapture.Plane` (`|GetArrayItem` _outactors_2)) false)
                    (for _array_element_4 (`SceneComponent.GetChildrenComponents` _array_element_3 false)
                      (if (`KismetStringLibrary.Contains` (`KismetSystemLibrary.GetDisplayName` _array_element_4) "MagnumAmmo")
                        (`SceneComponent.SetVisibility` _array_element_4 false false)
                        (set `/Game/GGProjectExamples/Blueprints/InventoryComponent.MagnumAmmoAdded` false (`/Game/GGProjectExamples/GothGirlCharacter/GothGirlCharacter.InventoryComponent` _asgoth_girl_character_4))
                        (else
                          (if (`KismetStringLibrary.EqualEqual_StrStr` _returnvalue "Uzis") :!label _label_2
                            (set `/Game/GGProjectExamples/GothGirlCharacter/GothGirlCharacter.HasUzis` true _asgoth_girl_character_2)
                            (bind _outactors_3 (`GameplayStatics.GetAllActorsOfClass` "/Game/GGProjectExamples/UserInterface/RenderTarget/3DMeshCapture.3DMeshCapture_C"))
                            (bind _asgoth_girl_character_5 (cast `/Game/GGProjectExamples/GothGirlCharacter/GothGirlCharacter` (`GameplayStatics.GetPlayerCharacter` 0)))
                            (for _array_element_5 (`SceneComponent.GetChildrenComponents` (`/Game/GGProjectExamples/UserInterface/RenderTarget/3DMeshCapture.Plane` (`|GetArrayItem` _outactors_3)) false)
                              (for _array_element_6 (`SceneComponent.GetChildrenComponents` _array_element_5 false)
                                (if (`KismetStringLibrary.Contains` (`KismetSystemLibrary.GetDisplayName` _array_element_6) "UziAmmo")
                                  (`SceneComponent.SetVisibility` _array_element_6 false false)
                                  (set `/Game/GGProjectExamples/Blueprints/InventoryComponent.UziAmmoAdded` false (`/Game/GGProjectExamples/GothGirlCharacter/GothGirlCharacter.InventoryComponent` _asgoth_girl_character_5))
                                  (else
                                    (if (`KismetStringLibrary.EqualEqual_StrStr` _returnvalue "Pistols") :!label _label_3
                                      (set `/Game/GGProjectExamples/GothGirlCharacter/GothGirlCharacter.HasPistols` true _asgoth_girl_character_2)
                                      (bind _outactors_4 (`GameplayStatics.GetAllActorsOfClass` "/Game/GGProjectExamples/UserInterface/RenderTarget/3DMeshCapture.3DMeshCapture_C"))
                                      (for _array_element_7 (`SceneComponent.GetChildrenComponents` (`/Game/GGProjectExamples/UserInterface/RenderTarget/3DMeshCapture.Plane` (`|GetArrayItem` _outactors_4)) false)
                                        (if true
                                          (bind _output (`|GetArrayItem` (`SceneComponent.GetChildrenComponents` _array_element_7 false) 1))
                                          (if (`KismetSystemLibrary.IsValid` _output)
                                            (`SceneComponent.SetVisibility` _output false false)
                                            (else
                                              (if _itemstructure_isconsumable :!label _label_4
                                                _
                                                (else
                                                  _))
                                              (bind _returnvalue_2 (`Character.PlayAnimMontage` _asgoth_girl_character_2 "/Game/GGProjectExamples/GothGirlCharacter/GothGirlRootModel/PickUp_Montage.PickUp_Montage" 1.0 "None"))
                                              (`KismetSystemLibrary.Delay` _returnvalue_2)
                                              (bind _success (`/Game/GGProjectExamples/Blueprints/InventoryComponent.AddToInventory` (`self.GetComponentByClass` Interacter "/Game/GGProjectExamples/Blueprints/InventoryComponent.InventoryComponent_C") (make `/Game/GGProjectExamples/Blueprints/SlotStructure` (make `/Game/GGProjectExamples/Blueprints/ItemStructure` "None" "None" _itemstructure_staticmesh_2 _itemstructure_thumbnail_2 _itemstructure_quantity 0.0 _itemstructure_class_2 true 9999 true false _itemstructure_ammo false false 0.0 _itemstructure_actor) _itemstructure_quantity)))
                                              (if _success
                                                (`self.K2_DestroyActor`)
                                                (bind _returnvalue_3 (`Character.PlayAnimMontage` _asgoth_girl_character_2 "/Game/GGProjectExamples/GothGirlCharacter/GothGirlRootModel/PickUp_Montage.PickUp_Montage" -1.0 "None"))
                                                (`KismetSystemLibrary.Delay` _returnvalue_3))))
                                          (else
                                            (goto _label_4))))
                                      (else
                                        (goto _label_4))))))
                              (goto _label_4))
                            (goto _label_4)
                            (else
                              (goto _label_3))))))
                    (goto _label_3))
                  (else
                    (goto _label_2))))))
          (goto _label))
        (else
          (goto _label))))))

(fn `UseItem`
  (returns (Success :type Boolean))
  (return false))

(fn `UserConstructionScript`)