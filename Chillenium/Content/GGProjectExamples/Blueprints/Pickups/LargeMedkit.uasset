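; Large Medkit item Blueprint that restores the player's health when used.
; UseItem runs the parent logic, then searches the GothGirlCharacter's inventory component for an entry matched by the hardcoded name "Large Medkit".
; The first match's HealingValue from its item structure is added to current health, clamped between zero and max, and the parent's result is returned.
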(fn `UseItem`
  (returns (Success :type Boolean))
  (bind _success (`parent.UseItem`))
  (bind _asgoth_girl_character (cast `/Game/GGProjectExamples/GothGirlCharacter/GothGirlCharacter` (`GameplayStatics.GetPlayerCharacter` 0)))
  (bind _asgoth_girl_character_2 (cast `/Game/GGProjectExamples/GothGirlCharacter/GothGirlCharacter` (`GameplayStatics.GetPlayerCharacter` 0)))
  (for _array_element (`/Game/GGProjectExamples/Blueprints/InventoryComponent.Inventory` (`/Game/GGProjectExamples/GothGirlCharacter/GothGirlCharacter.InventoryComponent` _asgoth_girl_character_2))
    (if (`KismetStringLibrary.EqualEqual_StrStr` "Large Medkit" (`KismetTextLibrary.Conv_TextToString` (break `/Game/GGProjectExamples/Blueprints/ItemStructure` (break `/Game/GGProjectExamples/Blueprints/SlotStructure` _array_element))))
      (set `/Game/GGProjectExamples/GothGirlCharacter/GothGirlCharacter.CurrentHealth` (`KismetMathLibrary.FClamp` (+ (`/Game/GGProjectExamples/GothGirlCharacter/GothGirlCharacter.CurrentHealth` _asgoth_girl_character) (`.HealingValue_43_AEB801F24567508F59584D9311FA36BE` (break `/Game/GGProjectExamples/Blueprints/ItemStructure` (break `/Game/GGProjectExamples/Blueprints/SlotStructure` _array_element)))) 0.0 (`/Game/GGProjectExamples/GothGirlCharacter/GothGirlCharacter.MaxHealth` _asgoth_girl_character)) _asgoth_girl_character)
      (return _success))))

(fn `UserConstructionScript`
  (`parent.UserConstructionScript`))