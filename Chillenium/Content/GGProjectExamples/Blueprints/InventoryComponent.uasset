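; Inventory component for the Goth Girl character that stores items in fixed slots and toggles a paused inventory window.
; PrepareInventory refills slots from class defaults while keeping quantities.
; AddToInventory fills partial stacks, recursing on overflow, or creates new ones.
; After stack merges, it updates the 3DMeshCapture item display with ammo meshes or visible items and can holster a spawned shotgun, logic that ReInit duplicates.
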(event `self.ReceiveBeginPlay`
  (`self.PrepareInventory`))

(event `PlayAnimation`)

(fn `AddToInventory`
  (params (ContentsToAdd :type "/Game/GGProjectExamples/Blueprints/SlotStructure Structure"))
  (returns (Success :type Boolean))
  (if (`.IsStackable_30_29E3E5DA4DFD6C7282D749A1DCD0CD99` (break `/Game/GGProjectExamples/Blueprints/ItemStructure` (break `/Game/GGProjectExamples/Blueprints/SlotStructure` ContentsToAdd)))
    (bind _stackindex (`self.HasPartialStack` (`local.ContentsToAdd`))
      (:`True`
        (bind _success (`self.AddToStack` (`local.ContentsToAdd`) _stackindex)))
      (:`False`
        (`self.CreateStack` (`local.ContentsToAdd`) :!label _label)))
    (else
      (goto _label)))
  (if _success
    (bind _asgoth_girl_character (cast `/Game/GGProjectExamples/GothGirlCharacter/GothGirlCharacter` (`GameplayStatics.GetPlayerCharacter` 0)))
    (for (_array_element _array_index) (`/Game/GGProjectExamples/Blueprints/InventoryComponent.Inventory` (`/Game/GGProjectExamples/GothGirlCharacter/GothGirlCharacter.InventoryComponent` _asgoth_girl_character))
      (if (> (`.Quantity_12_9950F2D440312310861AE6AE41510B5C` (break `/Game/GGProjectExamples/Blueprints/ItemStructure` (break `/Game/GGProjectExamples/Blueprints/SlotStructure` _array_element))) 0)
        (bind _outactors (`GameplayStatics.GetAllActorsOfClass` "/Game/GGProjectExamples/UserInterface/RenderTarget/3DMeshCapture.3DMeshCapture_C"))
        (bind _asgoth_girl_character_2 (cast `/Game/GGProjectExamples/GothGirlCharacter/GothGirlCharacter` (`GameplayStatics.GetPlayerCharacter` 0)))
        (bind _hasmagnums (`/Game/GGProjectExamples/GothGirlCharacter/GothGirlCharacter.HasMagnums` _asgoth_girl_character_2))
        (if (and (== "/Game/GGProjectExamples/Blueprints/Weapons/Magnums.Magnums_C" (`.Class_18_979DFC74474C1235986F07A63A082F86` (break `/Game/GGProjectExamples/Blueprints/ItemStructure` (break `/Game/GGProjectExamples/Blueprints/SlotStructure` _array_element)))) (not _hasmagnums) (not (`self.MagnumAmmoAdded`)))
          (bind _output (`|GetArrayItem` _outactors))
          (bind _returnvalue (`|AddComponentByClass` :`self` _output :`Class` "/Script/Engine.StaticMeshComponent" :`bManualAttachment` true))
          (`StaticMeshComponent.SetStaticMesh` _returnvalue "/Game/GGProjectExamples/Blueprints/Pickups/Meshes/MagnumAmmo.MagnumAmmo")
          (bind _output_2 (`|GetArrayItem` (`SceneComponent.GetChildrenComponents` (`/Game/GGProjectExamples/UserInterface/RenderTarget/3DMeshCapture.Plane` _output) false) _array_index))
          (`SceneComponent.K2_AttachToComponent` _returnvalue _output_2 "None" "SnapToTarget" "SnapToTarget" "SnapToTarget" true)
          (set `self.MagnumAmmoAdded` true))
        (bind _hasshotgun (`/Game/GGProjectExamples/GothGirlCharacter/GothGirlCharacter.HasShotgun` _asgoth_girl_character_2))
        (if (and (== "/Game/GGProjectExamples/Blueprints/Weapons/Shotgun.Shotgun_C" (`.Class_18_979DFC74474C1235986F07A63A082F86` (break `/Game/GGProjectExamples/Blueprints/ItemStructure` (break `/Game/GGProjectExamples/Blueprints/SlotStructure` _array_element)))) (not _hasshotgun) (not (`self.ShotgunAmmoAdded`))) :!label _label_2
          (bind _returnvalue_2 (`|AddComponentByClass` :`self` _output :`Class` "/Script/Engine.StaticMeshComponent" :`bManualAttachment` true))
          (`StaticMeshComponent.SetStaticMesh` _returnvalue_2 "/Game/GGProjectExamples/Blueprints/Pickups/Meshes/ShotgunAmmo.ShotgunAmmo")
          (`SceneComponent.K2_AttachToComponent` _returnvalue_2 _output_2 "None" "SnapToTarget" "SnapToTarget" "SnapToTarget" true)
          (set `self.ShotgunAmmoAdded` true)
          (goto _label_2)
          (else
            (bind _hasuzis (`/Game/GGProjectExamples/GothGirlCharacter/GothGirlCharacter.HasUzis` _asgoth_girl_character_2))
            (if (and (== "/Game/GGProjectExamples/Blueprints/Weapons/Uzis.Uzis_C" (`.Class_18_979DFC74474C1235986F07A63A082F86` (break `/Game/GGProjectExamples/Blueprints/ItemStructure` (break `/Game/GGProjectExamples/Blueprints/SlotStructure` _array_element)))) (not _hasuzis) (not (`self.UziAmmoAdded`)))
              (bind _returnvalue_3 (`|AddComponentByClass` :`self` _output :`Class` "/Script/Engine.StaticMeshComponent" :`bManualAttachment` true))
              (`StaticMeshComponent.SetStaticMesh` _returnvalue_3 "/Game/GGProjectExamples/Blueprints/Pickups/Meshes/UziAmmo.UziAmmo")
              (`SceneComponent.K2_AttachToComponent` _returnvalue_3 _output_2 "None" "SnapToTarget" "SnapToTarget" "SnapToTarget" true)
              (set `self.UziAmmoAdded` true))
            (bind _haspistols (`/Game/GGProjectExamples/GothGirlCharacter/GothGirlCharacter.HasPistols` _asgoth_girl_character_2))
            (if (and (== "/Game/GGProjectExamples/Blueprints/Weapons/Pistols.Pistols_C" (`.Class_18_979DFC74474C1235986F07A63A082F86` (break `/Game/GGProjectExamples/Blueprints/ItemStructure` (break `/Game/GGProjectExamples/Blueprints/SlotStructure` _array_element)))) (not _haspistols) false)
              (bind _returnvalue_4 (`|AddComponentByClass` :`self` _output :`Class` "/Script/Engine.StaticMeshComponent" :`bManualAttachment` true))
              (`StaticMeshComponent.SetStaticMesh` _returnvalue_4 "/Game/GGProjectExamples/Blueprints/Pickups/Meshes/GothGirlHolsters.GothGirlHolsters")
              (`SceneComponent.K2_AttachToComponent` _returnvalue_4 _output_2 "None" "SnapToTarget" "SnapToTarget" "SnapToTarget" true))
            (if (and (== (`.Class_18_979DFC74474C1235986F07A63A082F86` (break `/Game/GGProjectExamples/Blueprints/ItemStructure` (break `/Game/GGProjectExamples/Blueprints/SlotStructure` _array_element))) "/Game/GGProjectExamples/Blueprints/Weapons/Magnums.Magnums_C") _hasmagnums)
              (`SceneComponent.SetVisibility` _output_2 true false :!label _label_3)
              (elif (and (== (`.Class_18_979DFC74474C1235986F07A63A082F86` (break `/Game/GGProjectExamples/Blueprints/ItemStructure` (break `/Game/GGProjectExamples/Blueprints/SlotStructure` _array_element))) "/Game/GGProjectExamples/Blueprints/Weapons/Shotgun.Shotgun_C") _hasshotgun)
                (goto _label_3)
                (elif (and (== (`.Class_18_979DFC74474C1235986F07A63A082F86` (break `/Game/GGProjectExamples/Blueprints/ItemStructure` (break `/Game/GGProjectExamples/Blueprints/SlotStructure` _array_element))) "/Game/GGProjectExamples/Blueprints/Weapons/Uzis.Uzis_C") _hasuzis)
                  (goto _label_3)
                  (elif (and (== (`.Class_18_979DFC74474C1235986F07A63A082F86` (break `/Game/GGProjectExamples/Blueprints/ItemStructure` (break `/Game/GGProjectExamples/Blueprints/SlotStructure` _array_element))) "/Game/GGProjectExamples/Blueprints/Weapons/Pistols.Pistols_C") _haspistols)
                    (goto _label_3)
                    (elif (`.IsConsumable_24_8BA97FAD47108B1B5249EAACB9422910` (break `/Game/GGProjectExamples/Blueprints/ItemStructure` (break `/Game/GGProjectExamples/Blueprints/SlotStructure` _array_element)))
                      (goto _label_3)
                      (else
                        _))))))
            (if (>= _array_index 5)
              (`/Game/GGProjectExamples/GothGirlCharacter/GothGirlCharacter.ShotgunEquipped` _asgoth_girl_character_2
                (:`then`
                  _)
                (:`else`
                  (if (`/Game/GGProjectExamples/GothGirlCharacter/GothGirlCharacter.HasShotgun` _asgoth_girl_character_2)
                    (bind _returnvalue_5 (`|SpawnActorFromClass` "/Game/GGProjectExamples/Blueprints/Weapons/Shotgun.Shotgun_C" (`KismetMathLibrary.MakeTransform` (0.0 0.0 0.0)) "Undefined" "OverrideRootScale" null null))
                    (bind _output_get (set `/Game/GGProjectExamples/GothGirlCharacter/GothGirlCharacter.ShotgunEquipped` _returnvalue_5 _asgoth_girl_character_2))
                    (`PrimitiveComponent.SetCollisionEnabled` (`/Game/GGProjectExamples/Blueprints/Pickups/Item.ItemInteractCollision` _output_get) "NoCollision")
                    (`PrimitiveComponent.SetCollisionEnabled` (`/Game/GGProjectExamples/Blueprints/Pickups/Item.ItemRadius` _output_get) "NoCollision")
                    (`PrimitiveComponent.SetCollisionEnabled` (`/Game/GGProjectExamples/Blueprints/Pickups/Item.BaseMesh` _output_get) "NoCollision")
                    (`Actor.K2_AttachToComponent` _returnvalue_5 (`Character.Mesh` _asgoth_girl_character_2) "ShotgunHolster" "SnapToTarget" "SnapToTarget" "SnapToTarget" true)
                    (`Actor.K2_AttachToComponent` _output_get (`Character.Mesh` _asgoth_girl_character_2) "ShotgunHolster" "SnapToTarget" "SnapToTarget" "SnapToTarget" true))))
              (return true))))))
    (return true)))

(fn `AddToStack`
  (params (`Slot Structure` :type "/Game/GGProjectExamples/Blueprints/SlotStructure Structure") (`Slot Index` :type Integer))
  (returns (Success :type Boolean))
  (bind _inventory (`self.Inventory`))
  (bind _slot_structure_itemstructure (break `/Game/GGProjectExamples/Blueprints/SlotStructure` (`local.Slot Structure`)))
  (bind (_slot_structure_itemstructure_2 _slot_structure_quantity) (break `/Game/GGProjectExamples/Blueprints/SlotStructure` (`local.Slot Structure`)))
  (bind _slot_index (`local.Slot Index`))
  (bind _slot_structure (`local.Slot Structure`))
  (bind (_name _description _staticmesh _thumbnail _quantity _damage _class _isconsumable _maxstacksize) (break `/Game/GGProjectExamples/Blueprints/ItemStructure` _slot_structure_itemstructure))
  (bind _output (`|GetArrayItem` (`self.Inventory`) `Slot Index`))
  (bind _output_2 (`|GetArrayItem` _inventory _slot_index))
  (bind _output_get (set `self.currentQuantity` (`.Quantity_12_9950F2D440312310861AE6AE41510B5C` (break `/Game/GGProjectExamples/Blueprints/ItemStructure` (break `/Game/GGProjectExamples/Blueprints/SlotStructure` _output)))))
  (if (> (+ _output_get (`.Quantity_4_35298EC84C24FCFE8CF4C38B8C6F408F` (break `/Game/GGProjectExamples/Blueprints/SlotStructure` `Slot Structure`))) (`.MaxStackSize_29_6419EDD64F43EE932C1331A46F76FB29` (break `/Game/GGProjectExamples/Blueprints/ItemStructure` (break `/Game/GGProjectExamples/Blueprints/SlotStructure` _output))))
    (`KismetArrayLibrary.Array_Set` (`self.Inventory`) (`local.Slot Index`) (make `/Game/GGProjectExamples/Blueprints/SlotStructure` _slot_structure_itemstructure _maxstacksize))
    (`self.AddToInventory` (make `/Game/GGProjectExamples/Blueprints/SlotStructure` _slot_structure_itemstructure_2 (- _slot_structure_quantity (- _maxstacksize (`self.currentQuantity`)))))
    (else
      (`KismetArrayLibrary.Array_Set` _inventory _slot_index (make `/Game/GGProjectExamples/Blueprints/SlotStructure` (make `/Game/GGProjectExamples/Blueprints/ItemStructure` (break `/Game/GGProjectExamples/Blueprints/ItemStructure` (break `/Game/GGProjectExamples/Blueprints/SlotStructure` _output_2)) (`.Description_6_D10D354B4806A59A3040F2859B5DB4CD` (break `/Game/GGProjectExamples/Blueprints/ItemStructure` (break `/Game/GGProjectExamples/Blueprints/SlotStructure` _output_2))) (`.StaticMesh_9_F844FCE345E84D600F6E63B38081FA3A` (break `/Game/GGProjectExamples/Blueprints/ItemStructure` (break `/Game/GGProjectExamples/Blueprints/SlotStructure` _output_2))) (`.Thumbnail_21_141C497E44613DE0EDE9429D05701D00` (break `/Game/GGProjectExamples/Blueprints/ItemStructure` (break `/Game/GGProjectExamples/Blueprints/SlotStructure` _output_2))) (+ (`.Quantity_12_9950F2D440312310861AE6AE41510B5C` (break `/Game/GGProjectExamples/Blueprints/ItemStructure` (break `/Game/GGProjectExamples/Blueprints/SlotStructure` _output_2))) (`.Quantity_12_9950F2D440312310861AE6AE41510B5C` (break `/Game/GGProjectExamples/Blueprints/ItemStructure` (break `/Game/GGProjectExamples/Blueprints/SlotStructure` _slot_structure)))) (`.Damage_25_6E25309B4AD57ED9F26F7581310510DD` (break `/Game/GGProjectExamples/Blueprints/ItemStructure` (break `/Game/GGProjectExamples/Blueprints/SlotStructure` _output_2))) (`.Class_18_979DFC74474C1235986F07A63A082F86` (break `/Game/GGProjectExamples/Blueprints/ItemStructure` (break `/Game/GGProjectExamples/Blueprints/SlotStructure` _output_2))) (`.IsConsumable_24_8BA97FAD47108B1B5249EAACB9422910` (break `/Game/GGProjectExamples/Blueprints/ItemStructure` (break `/Game/GGProjectExamples/Blueprints/SlotStructure` _output_2))) (`.MaxStackSize_29_6419EDD64F43EE932C1331A46F76FB29` (break `/Game/GGProjectExamples/Blueprints/ItemStructure` (break `/Game/GGProjectExamples/Blueprints/SlotStructure` _slot_structure))) (`.IsStackable_30_29E3E5DA4DFD6C7282D749A1DCD0CD99` (break `/Game/GGProjectExamples/Blueprints/ItemStructure` (break `/Game/GGProjectExamples/Blueprints/SlotStructure` _output_2))) (`.IsPickable_32_48114AD04B061254B2DCFBB61C386029` (break `/Game/GGProjectExamples/Blueprints/ItemStructure` (break `/Game/GGProjectExamples/Blueprints/SlotStructure` _output_2))) (`.Ammo_35_F0E46CBA4658EF4A4C5F94BC77692BAE` (break `/Game/GGProjectExamples/Blueprints/ItemStructure` (break `/Game/GGProjectExamples/Blueprints/SlotStructure` _output_2))) (`.IsEquipped_38_4F813DB34A1B8F8044D7C1A452ED55CA` (break `/Game/GGProjectExamples/Blueprints/ItemStructure` (break `/Game/GGProjectExamples/Blueprints/SlotStructure` _output_2))) (`.HasWeapon_40_A00683E84A4CAE3032A7F1BF1D037E37` (break `/Game/GGProjectExamples/Blueprints/ItemStructure` (break `/Game/GGProjectExamples/Blueprints/SlotStructure` _output_2))) (`.HealingValue_43_AEB801F24567508F59584D9311FA36BE` (break `/Game/GGProjectExamples/Blueprints/ItemStructure` (break `/Game/GGProjectExamples/Blueprints/SlotStructure` _output_2))) (`.Actor_48_0D99C08E4992DC09B0C918B3590F9CC4` (break `/Game/GGProjectExamples/Blueprints/ItemStructure` (break `/Game/GGProjectExamples/Blueprints/SlotStructure` _output_2)))) (+ (`.Quantity_4_35298EC84C24FCFE8CF4C38B8C6F408F` (break `/Game/GGProjectExamples/Blueprints/SlotStructure` _output_2)) (`.Quantity_4_35298EC84C24FCFE8CF4C38B8C6F408F` (break `/Game/GGProjectExamples/Blueprints/SlotStructure` _slot_structure)))))))
  (return true))

(fn `CreateStack`
  (params (`Slot Structure` :type "/Game/GGProjectExamples/Blueprints/SlotStructure Structure"))
  (bind _inventory (`self.Inventory`))
  (`KismetArrayLibrary.Array_Set` _inventory (`KismetArrayLibrary.Array_Find` _inventory (make `/Game/GGProjectExamples/Blueprints/SlotStructure` (struct :`Name` "NSLOCTEXT(\"[D60A11164E6372AC8AC2E3BE69BA7974]\", \"29FC0C8145F3FF4762E26CB8FF55E163\", \"None\")" :`Description` "NSLOCTEXT(\"[D60A11164E6372AC8AC2E3BE69BA7974]\", \"B7C8B6944E1A5AFC9BCB26BFD6F0654A\", \"None\")" :`IsConsumable` true :`MaxStackSize` 4 :`IsStackable` true))) `Slot Structure`))

(fn `PrepareInventory`
  (`KismetArrayLibrary.Array_Resize` (`self.Inventory`) (`self.NumberOfSlots`))
  (for (_array_element _array_index) (`self.Inventory`)
    (bind (_name _description _staticmesh _thumbnail _quantity _damage _class) (break `/Game/GGProjectExamples/Blueprints/ItemStructure` (break `/Game/GGProjectExamples/Blueprints/SlotStructure` _array_element)))
    (if (!= _class null)
      (bind _itemstructure (defaults `Object` _class))
      (`KismetArrayLibrary.Array_Set` (`self.Inventory`) _array_index (make `/Game/GGProjectExamples/Blueprints/SlotStructure` (make `/Game/GGProjectExamples/Blueprints/ItemStructure` (break `/Game/GGProjectExamples/Blueprints/ItemStructure` _itemstructure) (`.Description_6_D10D354B4806A59A3040F2859B5DB4CD` (break `/Game/GGProjectExamples/Blueprints/ItemStructure` _itemstructure)) (`.StaticMesh_9_F844FCE345E84D600F6E63B38081FA3A` (break `/Game/GGProjectExamples/Blueprints/ItemStructure` _itemstructure)) (`.Thumbnail_21_141C497E44613DE0EDE9429D05701D00` (break `/Game/GGProjectExamples/Blueprints/ItemStructure` _itemstructure)) _quantity (`.Damage_25_6E25309B4AD57ED9F26F7581310510DD` (break `/Game/GGProjectExamples/Blueprints/ItemStructure` _itemstructure)) (`.Class_18_979DFC74474C1235986F07A63A082F86` (break `/Game/GGProjectExamples/Blueprints/ItemStructure` _itemstructure)) (`.IsConsumable_24_8BA97FAD47108B1B5249EAACB9422910` (break `/Game/GGProjectExamples/Blueprints/ItemStructure` _itemstructure)) (`.MaxStackSize_29_6419EDD64F43EE932C1331A46F76FB29` (break `/Game/GGProjectExamples/Blueprints/ItemStructure` _itemstructure)) (`.IsStackable_30_29E3E5DA4DFD6C7282D749A1DCD0CD99` (break `/Game/GGProjectExamples/Blueprints/ItemStructure` _itemstructure)) (`.IsPickable_32_48114AD04B061254B2DCFBB61C386029` (break `/Game/GGProjectExamples/Blueprints/ItemStructure` _itemstructure)) (`.Ammo_35_F0E46CBA4658EF4A4C5F94BC77692BAE` (break `/Game/GGProjectExamples/Blueprints/ItemStructure` _itemstructure)) (`.IsEquipped_38_4F813DB34A1B8F8044D7C1A452ED55CA` (break `/Game/GGProjectExamples/Blueprints/ItemStructure` _itemstructure)) (`.HasWeapon_40_A00683E84A4CAE3032A7F1BF1D037E37` (break `/Game/GGProjectExamples/Blueprints/ItemStructure` _itemstructure)) (`.HealingValue_43_AEB801F24567508F59584D9311FA36BE` (break `/Game/GGProjectExamples/Blueprints/ItemStructure` _itemstructure)) (`.Actor_48_0D99C08E4992DC09B0C918B3590F9CC4` (break `/Game/GGProjectExamples/Blueprints/ItemStructure` _itemstructure))) (`.Quantity_4_35298EC84C24FCFE8CF4C38B8C6F408F` (break `/Game/GGProjectExamples/Blueprints/SlotStructure` _array_element)))))))

(fn `ReInit`
  (returns (Success :type Boolean))
  (bind _asgoth_girl_character (cast `/Game/GGProjectExamples/GothGirlCharacter/GothGirlCharacter` (`GameplayStatics.GetPlayerCharacter` 0)))
  (for (_array_element _array_index) (`/Game/GGProjectExamples/Blueprints/InventoryComponent.Inventory` (`/Game/GGProjectExamples/GothGirlCharacter/GothGirlCharacter.InventoryComponent` _asgoth_girl_character))
    (if (> (`.Quantity_12_9950F2D440312310861AE6AE41510B5C` (break `/Game/GGProjectExamples/Blueprints/ItemStructure` (break `/Game/GGProjectExamples/Blueprints/SlotStructure` _array_element))) 0)
      (bind _outactors (`GameplayStatics.GetAllActorsOfClass` "/Game/GGProjectExamples/UserInterface/RenderTarget/3DMeshCapture.3DMeshCapture_C"))
      (bind _asgoth_girl_character_2 (cast `/Game/GGProjectExamples/GothGirlCharacter/GothGirlCharacter` (`GameplayStatics.GetPlayerCharacter` 0)))
      (bind _hasmagnums (`/Game/GGProjectExamples/GothGirlCharacter/GothGirlCharacter.HasMagnums` _asgoth_girl_character_2))
      (if (and (== "/Game/GGProjectExamples/Blueprints/Weapons/Magnums.Magnums_C" (`.Class_18_979DFC74474C1235986F07A63A082F86` (break `/Game/GGProjectExamples/Blueprints/ItemStructure` (break `/Game/GGProjectExamples/Blueprints/SlotStructure` _array_element)))) (not _hasmagnums) (not (`self.MagnumAmmoAdded`)))
        (bind _output (`|GetArrayItem` _outactors))
        (bind _returnvalue (`|AddComponentByClass` :`self` _output :`Class` "/Script/Engine.StaticMeshComponent" :`bManualAttachment` true))
        (`StaticMeshComponent.SetStaticMesh` _returnvalue "/Game/GGProjectExamples/Blueprints/Pickups/Meshes/MagnumAmmo.MagnumAmmo")
        (bind _output_2 (`|GetArrayItem` (`SceneComponent.GetChildrenComponents` (`/Game/GGProjectExamples/UserInterface/RenderTarget/3DMeshCapture.Plane` _output) false) _array_index))
        (`SceneComponent.K2_AttachToComponent` _returnvalue _output_2 "None" "SnapToTarget" "SnapToTarget" "SnapToTarget" true)
        (set `self.MagnumAmmoAdded` true))
      (bind _hasshotgun (`/Game/GGProjectExamples/GothGirlCharacter/GothGirlCharacter.HasShotgun` _asgoth_girl_character_2))
      (if (and (== "/Game/GGProjectExamples/Blueprints/Weapons/Shotgun.Shotgun_C" (`.Class_18_979DFC74474C1235986F07A63A082F86` (break `/Game/GGProjectExamples/Blueprints/ItemStructure` (break `/Game/GGProjectExamples/Blueprints/SlotStructure` _array_element)))) (not _hasshotgun) (not (`self.ShotgunAmmoAdded`))) :!label _label
        (bind _returnvalue_2 (`|AddComponentByClass` :`self` _output :`Class` "/Script/Engine.StaticMeshComponent" :`bManualAttachment` true))
        (`StaticMeshComponent.SetStaticMesh` _returnvalue_2 "/Game/GGProjectExamples/Blueprints/Pickups/Meshes/ShotgunAmmo.ShotgunAmmo")
        (`SceneComponent.K2_AttachToComponent` _returnvalue_2 _output_2 "None" "SnapToTarget" "SnapToTarget" "SnapToTarget" true)
        (set `self.ShotgunAmmoAdded` true)
        (goto _label)
        (else
          (bind _hasuzis (`/Game/GGProjectExamples/GothGirlCharacter/GothGirlCharacter.HasUzis` _asgoth_girl_character_2))
          (if (and (== "/Game/GGProjectExamples/Blueprints/Weapons/Uzis.Uzis_C" (`.Class_18_979DFC74474C1235986F07A63A082F86` (break `/Game/GGProjectExamples/Blueprints/ItemStructure` (break `/Game/GGProjectExamples/Blueprints/SlotStructure` _array_element)))) (not _hasuzis) (not (`self.UziAmmoAdded`)))
            (bind _returnvalue_3 (`|AddComponentByClass` :`self` _output :`Class` "/Script/Engine.StaticMeshComponent" :`bManualAttachment` true))
            (`StaticMeshComponent.SetStaticMesh` _returnvalue_3 "/Game/GGProjectExamples/Blueprints/Pickups/Meshes/UziAmmo.UziAmmo")
            (`SceneComponent.K2_AttachToComponent` _returnvalue_3 _output_2 "None" "SnapToTarget" "SnapToTarget" "SnapToTarget" true)
            (set `self.UziAmmoAdded` true))
          (bind _haspistols (`/Game/GGProjectExamples/GothGirlCharacter/GothGirlCharacter.HasPistols` _asgoth_girl_character_2))
          (if (and (== "/Game/GGProjectExamples/Blueprints/Weapons/Pistols.Pistols_C" (`.Class_18_979DFC74474C1235986F07A63A082F86` (break `/Game/GGProjectExamples/Blueprints/ItemStructure` (break `/Game/GGProjectExamples/Blueprints/SlotStructure` _array_element)))) (not _haspistols) false)
            (bind _returnvalue_4 (`|AddComponentByClass` :`self` _output :`Class` "/Script/Engine.StaticMeshComponent" :`bManualAttachment` true))
            (`StaticMeshComponent.SetStaticMesh` _returnvalue_4 "/Game/GGProjectExamples/Blueprints/Pickups/Meshes/GothGirlHolsters.GothGirlHolsters")
            (`SceneComponent.K2_AttachToComponent` _returnvalue_4 _output_2 "None" "SnapToTarget" "SnapToTarget" "SnapToTarget" true))
          (if (and (== (`.Class_18_979DFC74474C1235986F07A63A082F86` (break `/Game/GGProjectExamples/Blueprints/ItemStructure` (break `/Game/GGProjectExamples/Blueprints/SlotStructure` _array_element))) "/Game/GGProjectExamples/Blueprints/Weapons/Magnums.Magnums_C") _hasmagnums)
            (`SceneComponent.SetVisibility` _output_2 true false :!label _label_2)
            (elif (and (== (`.Class_18_979DFC74474C1235986F07A63A082F86` (break `/Game/GGProjectExamples/Blueprints/ItemStructure` (break `/Game/GGProjectExamples/Blueprints/SlotStructure` _array_element))) "/Game/GGProjectExamples/Blueprints/Weapons/Shotgun.Shotgun_C") _hasshotgun)
              (goto _label_2)
              (elif (and (== (`.Class_18_979DFC74474C1235986F07A63A082F86` (break `/Game/GGProjectExamples/Blueprints/ItemStructure` (break `/Game/GGProjectExamples/Blueprints/SlotStructure` _array_element))) "/Game/GGProjectExamples/Blueprints/Weapons/Uzis.Uzis_C") _hasuzis)
                (goto _label_2)
                (elif (and (== (`.Class_18_979DFC74474C1235986F07A63A082F86` (break `/Game/GGProjectExamples/Blueprints/ItemStructure` (break `/Game/GGProjectExamples/Blueprints/SlotStructure` _array_element))) "/Game/GGProjectExamples/Blueprints/Weapons/Pistols.Pistols_C") _haspistols)
                  (goto _label_2)
                  (elif (`.IsConsumable_24_8BA97FAD47108B1B5249EAACB9422910` (break `/Game/GGProjectExamples/Blueprints/ItemStructure` (break `/Game/GGProjectExamples/Blueprints/SlotStructure` _array_element)))
                    (goto _label_2)
                    (else
                      _))))))
          (if (>= _array_index 5)
            (`/Game/GGProjectExamples/GothGirlCharacter/GothGirlCharacter.ShotgunEquipped` _asgoth_girl_character_2
              (:`then`
                _)
              (:`else`
                (if (`/Game/GGProjectExamples/GothGirlCharacter/GothGirlCharacter.HasShotgun` _asgoth_girl_character_2)
                  (bind _returnvalue_5 (`|SpawnActorFromClass` "/Game/GGProjectExamples/Blueprints/Weapons/Shotgun.Shotgun_C" (`KismetMathLibrary.MakeTransform` (0.0 0.0 0.0)) "Undefined" "OverrideRootScale" null null))
                  (bind _output_get (set `/Game/GGProjectExamples/GothGirlCharacter/GothGirlCharacter.ShotgunEquipped` _returnvalue_5 _asgoth_girl_character_2))
                  (`PrimitiveComponent.SetCollisionEnabled` (`/Game/GGProjectExamples/Blueprints/Pickups/Item.ItemInteractCollision` _output_get) "NoCollision")
                  (`PrimitiveComponent.SetCollisionEnabled` (`/Game/GGProjectExamples/Blueprints/Pickups/Item.ItemRadius` _output_get) "NoCollision")
                  (`PrimitiveComponent.SetCollisionEnabled` (`/Game/GGProjectExamples/Blueprints/Pickups/Item.BaseMesh` _output_get) "NoCollision")
                  (`Actor.K2_AttachToComponent` _returnvalue_5 (`Character.Mesh` _asgoth_girl_character_2) "ShotgunHolster" "SnapToTarget" "SnapToTarget" "SnapToTarget" true)
                  (`Actor.K2_AttachToComponent` _output_get (`Character.Mesh` _asgoth_girl_character_2) "ShotgunHolster" "SnapToTarget" "SnapToTarget" "SnapToTarget" true))))
            (return true))))))
  (return true))

(fn `ToggleInventory`
  (bind _returnvalue (`GameplayStatics.GetPlayerController` 0))
  (bind _returnvalue_2 (`GameplayStatics.GetPlayerController` 0))
  (`self.InventoryWindow`
    (:`then`
      (`Widget.RemoveFromParent` (`self.InventoryWindow`))
      (set `self.InventoryWindow` null)
      (`WidgetBlueprintLibrary.SetInputMode_GameOnly` _returnvalue_2)
      (set `PlayerController.bShowMouseCursor` false _returnvalue_2)
      (bind _outactors (`GameplayStatics.GetAllActorsOfClass` null))
      (bind _asgoth_girl_character (cast `/Game/GGProjectExamples/GothGirlCharacter/GothGirlCharacter` (`|GetArrayItem` _outactors)))
      (set `/Game/GGProjectExamples/GothGirlCharacter/GothGirlCharacter.InInventory` false _asgoth_girl_character)
      (`GameplayStatics.SetGamePaused` false))
    (:`else`
      (`self.PrepareInventory`)
      (bind _returnvalue_3 (`|CreateWidget` "/Game/GGProjectExamples/UserInterface/InventoryWindow.InventoryWindow_C" null self))
      (set `self.InventoryWindow` _returnvalue_3)
      (bind _asgoth_girl_player_controller (cast `/Game/GGProjectExamples/Blueprints/GothGirlPlayerController` (`GameplayStatics.GetPlayerController` 0)))
      (bind _returnvalue_4 (`CanvasPanel.AddChildToCanvas` (`/Game/GGProjectExamples/UserInterface/HUD.HudCanvas` (`/Game/GGProjectExamples/Blueprints/GothGirlPlayerController.HudWidget` _asgoth_girl_player_controller)) (`self.InventoryWindow`)))
      (`CanvasPanelSlot.SetAutoSize` _returnvalue_4 true)
      (`CanvasPanelSlot.SetAlignment` _returnvalue_4 (0.5 0.5))
      (`CanvasPanelSlot.SetAnchors` _returnvalue_4 (`self.Anchors`))
      (`CanvasPanelSlot.SetPosition` _returnvalue_4 (`self.Position`))
      (`WidgetBlueprintLibrary.SetInputMode_GameAndUIEx` _returnvalue (`self.InventoryWindow`) "LockAlways" false)
      (set `PlayerController.bShowMouseCursor` true _returnvalue)
      (bind _outactors_2 (`GameplayStatics.GetAllActorsOfClass` "/Game/GGProjectExamples/GothGirlCharacter/GothGirlCharacter.GothGirlCharacter_C"))
      (bind _asgoth_girl_character_2 (cast `/Game/GGProjectExamples/GothGirlCharacter/GothGirlCharacter` (`|GetArrayItem` _outactors_2)))
      (set `/Game/GGProjectExamples/GothGirlCharacter/GothGirlCharacter.InInventory` true _asgoth_girl_character_2)
      (`GameplayStatics.SetGamePaused` true))))