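; Trigger-driven camera actor that takes over the view when GothGirlCharacter overlaps StartCamera and blends back at EndCamera.
; While it is the view target, Tick turns the camera toward the player when stationary, otherwise moves the spring arm with optional look-at rotation.
; Movement uses a per-axis TrackPlayer mask and a once-captured offset, printing debug values.
; TrackPoint disables tracking and shows this camera for two seconds before returning to the character.
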(event `self.ReceiveTick`
  (params (DeltaSeconds :type "Float (single-precision)"))
  (if (`self.ManualTrigger`)
    _
    (elif (== (`Controller.GetViewTarget` (`GameplayStatics.GetPlayerController` 0)) self)
      (if (`self.IsStationary`)
        (bind _rotation (`self.TrackPlayerRotation` DeltaSeconds))
        (`SceneComponent.K2_SetWorldRotation` (`self.Camera`) _rotation false false)
        (else
          (set `SpringArmComponent.bDoCollisionTest` false (`self.SpringArm`))
          (if (`self.NoRotation`)
            (bind _vector (`self.TrackPlayerMovement` DeltaSeconds))
            (`SceneComponent.K2_SetWorldLocation` (`self.SpringArm`) _vector false false)
            (else
              (bind _vector_2 (`self.TrackPlayerMovement` 0.0))
              (`SceneComponent.K2_SetWorldLocation` (`self.SpringArm`) _vector_2 false false)
              (bind _rotation_2 (`self.TrackPlayerRotation` 0.0))
              (`SceneComponent.K2_SetWorldRotation` (`self.Camera`) _rotation_2 false false))))))))

(event `Track Point`
  (set `self.ManualTrigger` true)
  (`PlayerController.SetViewTargetWithBlend` (`GameplayStatics.GetPlayerController` 0) self 0.0 "VTBlend_Linear" 0.0 false)
  (bind _asgoth_girl_character (cast `/Game/GGProjectExamples/GothGirlCharacter/GothGirlCharacter` (`GameplayStatics.GetPlayerCharacter` 0)))
  (`KismetSystemLibrary.Delay` 2.0)
  (`PlayerController.SetViewTargetWithBlend` (`GameplayStatics.GetPlayerController` 0) _asgoth_girl_character 0.0 "VTBlend_Linear" 0.0 false))

(event `self.StartCamera.OnComponentBeginOverlap`
  (params (OverlappedComponent :type "PrimitiveComponent Object Reference") (OtherActor :type "Actor Object Reference") (OtherComp :type "PrimitiveComponent Object Reference") (OtherBodyIndex :type Integer) (bFromSweep :type Boolean) (SweepResult :type "HitResult Structure (by ref)"))
  (cast `/Game/GGProjectExamples/GothGirlCharacter/GothGirlCharacter` OtherActor)
  (`PlayerController.SetViewTargetWithBlend` (`GameplayStatics.GetPlayerController` 0) self (`self.BlendTime`) "VTBlend_Linear" 0.0 false)
  (`/Engine/EditorBlueprintResources/StandardMacros.DoOnce` false
    (:`Completed`
      (set `self.Offset` (- (`SceneComponent.K2_GetComponentLocation` (`self.SpringArm`)) (`self.K2_GetActorLocation` (`GameplayStatics.GetPlayerCharacter` 0)))))))

(event `self.EndCamera.OnComponentBeginOverlap`
  (params (OverlappedComponent :type "PrimitiveComponent Object Reference") (OtherActor :type "Actor Object Reference") (OtherComp :type "PrimitiveComponent Object Reference") (OtherBodyIndex :type Integer) (bFromSweep :type Boolean) (SweepResult :type "HitResult Structure (by ref)"))
  (bind _asgoth_girl_character (cast `/Game/GGProjectExamples/GothGirlCharacter/GothGirlCharacter` OtherActor))
  (`PlayerController.SetViewTargetWithBlend` (`GameplayStatics.GetPlayerController` 0) _asgoth_girl_character (`self.BlendTime`) "VTBlend_Linear" 0.0 false))

(fn `TrackPlayerMovement`
  (params (DeltaTime :type "Float (double-precision)"))
  (returns (Vector :type "Vector Structure"))
  (bind _returnvalue (- (`self.K2_GetActorLocation`) (`self.Offset`)))
  (bind _returnvalue_2 (`self.K2_GetActorLocation` (`GameplayStatics.GetPlayerCharacter` 0)))
  (bind (_returnvalue_x _returnvalue_y) (`KismetMathLibrary.BreakVector` (`self.K2_GetActorLocation` (`GameplayStatics.GetPlayerCharacter` 0))))
  (bind (_returnvalue_x_2 _returnvalue_y_2 _returnvalue_z) (`KismetMathLibrary.BreakVector` (+ (* _returnvalue_2 (`self.TrackPlayer`)) (* _returnvalue (- (1.0 1.0 1.0) (`self.TrackPlayer`))))))
  (bind _returnvalue_3 (+ _returnvalue_x_2 _returnvalue_y))
  (`KismetSystemLibrary.PrintString` (`KismetStringLibrary.Conv_VectorToString` _returnvalue) true true (struct :`R` 1.0 :`B` 0.034148 :`A` 1.0))
  (`KismetSystemLibrary.PrintString` (`KismetStringLibrary.Conv_DoubleToString` _returnvalue_3))
  (`KismetSystemLibrary.PrintString` (`KismetStringLibrary.Conv_VectorToString` _returnvalue_2) true true (struct :`G` 1.0 :`B` 0.039178 :`A` 1.0))
  (return (`KismetMathLibrary.VInterpTo` _returnvalue (`KismetMathLibrary.MakeVector` _returnvalue_x_2 _returnvalue_3 _returnvalue_z) DeltaTime)))

(fn `TrackPlayerRotation`
  (params (DeltaTime :type "Float (double-precision)"))
  (returns (Rotation :type "Rotator Structure"))
  (return (`KismetMathLibrary.FindLookAtRotation` (`SceneComponent.K2_GetComponentLocation` (`self.Camera`)) (`self.K2_GetActorLocation` (`GameplayStatics.GetPlayerCharacter` 0)))))

(fn `UserConstructionScript`)