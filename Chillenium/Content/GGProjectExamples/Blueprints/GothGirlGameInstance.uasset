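; Game instance that manages save slots for player state and per-level data.
; LoadGame loads or creates the slot's save object, starting a looping AutoSave timer only for existing saves.
; SavePlayerData writes the slot before copying inventory, transform, health and weapon flags into the save object; LoadPlayerData applies them to GothGirlCharacter.
; Separate LevelDataObject saves use the level name as slot, with helpers to retrieve or delete player saves.
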(event `LoadGame`
  (params (SaveSlotName :type String))
  (bind _output_get (set `self.SaveSlotName` SaveSlotName))
  (bind _returnvalue (`GameplayStatics.DoesSaveGameExist` _output_get))
  (if _returnvalue
    (bind _returnvalue_2 (`GameplayStatics.LoadGameFromSlot` (`self.SaveSlotName`)))
    (bind _assave_game_object (cast `/Game/GGProjectExamples/Blueprints/SaveGameObject` _returnvalue_2))
    (set `self.SaveGameData` _assave_game_object)
    (`KismetSystemLibrary.K2_SetTimer` self "AutoSave" (`self.AutoSaveTimer`) true)
    (else
      (bind _returnvalue_3 (`GameplayStatics.CreateSaveGameObject` "/Game/GGProjectExamples/Blueprints/SaveGameObject.SaveGameObject_C"))
      (set `self.SaveGameData` _returnvalue_3))))

(fn `AutoSave`
  (`self.SavePlayerData`))

(fn `ClearSaveData`
  (`GameplayStatics.DeleteGameInSlot` (`self.SaveSlotName`)))

(fn `InitLevelSaveData`
  (bind _returnvalue (`GameplayStatics.GetCurrentLevelName` true))
  (bind _returnvalue_2 (`GameplayStatics.DoesSaveGameExist` _returnvalue))
  (if _returnvalue_2
    (bind _returnvalue_3 (`GameplayStatics.GetCurrentLevelName` true))
    (bind _returnvalue_4 (`GameplayStatics.LoadGameFromSlot` _returnvalue_3))
    (bind _aslevel_data_object (cast `/Game/GGProjectExamples/Blueprints/LevelDataObject` _returnvalue_4))
    (set `self.LevelSaveObject` _aslevel_data_object)
    (else
      (bind _returnvalue_5 (`GameplayStatics.CreateSaveGameObject` "/Game/GGProjectExamples/Blueprints/LevelDataObject.LevelDataObject_C"))
      (set `self.LevelSaveObject` _returnvalue_5))))

(fn `InitSlotSaveData`
  (bind _saveslotname (`self.SaveSlotName`))
  (`KismetSystemLibrary.PrintString` _saveslotname)
  (bind _returnvalue (`GameplayStatics.DoesSaveGameExist` _saveslotname))
  (if (not _returnvalue)
    (bind _returnvalue_2 (`GameplayStatics.CreateSaveGameObject` "/Game/GGProjectExamples/Blueprints/SaveGameObject.SaveGameObject_C"))
    (set `self.SaveGameData` _returnvalue_2)))

(fn `LoadPlayerData`
  (locals (PlayerReference :type "/Game/GGProjectExamples/GothGirlCharacter/GothGirlCharacter Object Reference"))
  (bind _playerreference (`local.PlayerReference`))
  (bind _savegamedata (`self.SaveGameData`))
  (bind _asgoth_girl_character (cast `/Game/GGProjectExamples/GothGirlCharacter/GothGirlCharacter` (`GameplayStatics.GetPlayerCharacter` 0)))
  (set `local.PlayerReference` _asgoth_girl_character)
  (for (_array_element _array_index) (`/Game/GGProjectExamples/Blueprints/SaveGameObject.SavedInventory` (`self.SaveGameData`))
    (bind _inventorycomponent (`/Game/GGProjectExamples/GothGirlCharacter/GothGirlCharacter.InventoryComponent` _asgoth_girl_character))
    (`KismetArrayLibrary.Array_Set` (`/Game/GGProjectExamples/Blueprints/InventoryComponent.Inventory` _inventorycomponent) _array_index _array_element)
    (`|ExecutionSequence`
      (:`then_0`
        (`Actor.K2_SetActorLocation` _playerreference (`/Game/GGProjectExamples/Blueprints/SaveGameObject.PlayerLocation` _savegamedata) false false))
      (:`then_1`
        (`Actor.K2_SetActorRotation` _playerreference (`/Game/GGProjectExamples/Blueprints/SaveGameObject.PlayerRotation` _savegamedata) false))
      (:`then_2`
        (set `/Game/GGProjectExamples/GothGirlCharacter/GothGirlCharacter.CurrentHealth` (`/Game/GGProjectExamples/Blueprints/SaveGameObject.PlayerHealth` _savegamedata) _playerreference))
      (:`then_3`
        (set `/Game/GGProjectExamples/GothGirlCharacter/GothGirlCharacter.HasPistols` (`/Game/GGProjectExamples/Blueprints/SaveGameObject.HasPistols` _savegamedata) _playerreference))
      (:`then_4`
        (set `/Game/GGProjectExamples/GothGirlCharacter/GothGirlCharacter.HasShotgun` (`/Game/GGProjectExamples/Blueprints/SaveGameObject.HasShotgun` _savegamedata) _playerreference))
      (:`then_5`
        (set `/Game/GGProjectExamples/GothGirlCharacter/GothGirlCharacter.HasMagnums` (`/Game/GGProjectExamples/Blueprints/SaveGameObject.HasMagnums` _savegamedata) _playerreference))
      (:`then_6`
        (set `/Game/GGProjectExamples/GothGirlCharacter/GothGirlCharacter.HasUzis` (`/Game/GGProjectExamples/Blueprints/SaveGameObject.HasUzis` _savegamedata) _playerreference))
      (:`then_8`
        (`/Game/GGProjectExamples/Blueprints/InventoryComponent.ReInit` _inventorycomponent)))))

(fn `RetrieveSaveData`
  (params (LocalSaveSlotName :type String))
  (returns (PlayerData :type "/Game/GGProjectExamples/Blueprints/PlayerSaveData Structure"))
  (bind _returnvalue (`GameplayStatics.DoesSaveGameExist` LocalSaveSlotName))
  (if _returnvalue
    (bind _returnvalue_2 (`GameplayStatics.LoadGameFromSlot` (`local.LocalSaveSlotName`)))
    (bind _assave_game_object (cast `/Game/GGProjectExamples/Blueprints/SaveGameObject` _returnvalue_2))
    (return (`/Game/GGProjectExamples/Blueprints/SaveGameObject.PlayerData` _assave_game_object))))

(fn `SaveLevelData`
  (bind _returnvalue (`GameplayStatics.GetCurrentLevelName` true))
  (`GameplayStatics.SaveGameToSlot` (`self.LevelSaveObject`) _returnvalue))

(fn `SavePlayerData`
  (locals (`Player Reference` :type "/Game/GGProjectExamples/GothGirlCharacter/GothGirlCharacter Object Reference"))
  (bind _player_reference (`local.Player Reference`))
  (bind _savegamedata (`self.SaveGameData`))
  (bind _savegamedata_2 (`self.SaveGameData`))
  (bind _savedinventory (`/Game/GGProjectExamples/Blueprints/SaveGameObject.SavedInventory` _savegamedata_2))
  (`self.InitSlotSaveData`)
  (bind _asgoth_girl_character (cast `/Game/GGProjectExamples/GothGirlCharacter/GothGirlCharacter` (`GameplayStatics.GetPlayerCharacter` 0)))
  (set `local.Player Reference` _asgoth_girl_character)
  (bind _returnvalue (`GameplayStatics.GetCurrentLevelName` true))
  (set `/Game/GGProjectExamples/Blueprints/SaveGameObject.LastLevelLoaded` _returnvalue _savegamedata_2)
  (bind _returnvalue_2 (`GameplayStatics.SaveGameToSlot` _savegamedata_2 (`self.SaveSlotName`)))
  (`KismetSystemLibrary.PrintString` (`KismetStringLibrary.Conv_BoolToString` _returnvalue_2))
  (`KismetArrayLibrary.Array_Resize` _savedinventory 6)
  (for (_array_element _array_index) (`/Game/GGProjectExamples/Blueprints/InventoryComponent.Inventory` (`/Game/GGProjectExamples/GothGirlCharacter/GothGirlCharacter.InventoryComponent` _asgoth_girl_character))
    (`KismetArrayLibrary.Array_Set` _savedinventory _array_index _array_element))
  (`|ExecutionSequence`
    (:`then_0`
      (set `/Game/GGProjectExamples/Blueprints/SaveGameObject.PlayerLocation` (`Actor.K2_GetActorLocation` _player_reference) _savegamedata))
    (:`then_1`
      (set `/Game/GGProjectExamples/Blueprints/SaveGameObject.PlayerRotation` (`Actor.K2_GetActorRotation` _player_reference) _savegamedata))
    (:`then_2`
      (set `/Game/GGProjectExamples/Blueprints/SaveGameObject.PlayerHealth` (`/Game/GGProjectExamples/GothGirlCharacter/GothGirlCharacter.CurrentHealth` _player_reference) _savegamedata))
    (:`then_3`
      (set `/Game/GGProjectExamples/Blueprints/SaveGameObject.HasPistols` (`/Game/GGProjectExamples/GothGirlCharacter/GothGirlCharacter.HasPistols` _player_reference) _savegamedata))
    (:`then_4`
      (set `/Game/GGProjectExamples/Blueprints/SaveGameObject.HasShotgun` (`/Game/GGProjectExamples/GothGirlCharacter/GothGirlCharacter.HasShotgun` _player_reference) _savegamedata))
    (:`then_5`
      (set `/Game/GGProjectExamples/Blueprints/SaveGameObject.HasMagnums` (`/Game/GGProjectExamples/GothGirlCharacter/GothGirlCharacter.HasMagnums` _player_reference) _savegamedata))
    (:`then_6`
      (set `/Game/GGProjectExamples/Blueprints/SaveGameObject.HasUzis` (`/Game/GGProjectExamples/GothGirlCharacter/GothGirlCharacter.HasUzis` _player_reference) _savegamedata))
    (:`then_7`
      (bind _returnvalue_3 (`GameplayStatics.GetCurrentLevelName` true))
      (set `/Game/GGProjectExamples/Blueprints/SaveGameObject.LastLevelLoaded` _returnvalue_3 (`self.LevelSaveObject`)))
    (:`then_8`
      (`KismetSystemLibrary.PrintString` "In the Middle of Saving" true true (struct :`R` 1.0 :`G` 0.52583 :`A` 1.0)))))