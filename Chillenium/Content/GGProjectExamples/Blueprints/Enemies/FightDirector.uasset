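; Fight director that coordinates enemy attacks by choosing which enemy in its list attacks the player.
; A looping four-second timer regrades enemies by how directly their forward vector opposes the player's, then tells the top-graded enemy's TestEnemy_AI controller to attack.
; The attacker then gets a random grade, which the next positional rescore overwrites.
; Each enemy carries a debug widget showing its grade, refreshed only for the attacker.
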(event `self.ReceiveBeginPlay`
  (for _array_element (`self.EnemyList`)
    (`self.AddDebugWidgets` _array_element))
  (`KismetSystemLibrary.K2_SetTimerDelegate` (delegate `TriggerAttack`) 4.0 true))

(event `TriggerAttack`
  (`self.RecalculateGrades`)
  (bind (_loc_highestvalue1 _loc_highestgradedai1) (`self.FindHighestGrade`))
  (bind _astest_enemy_ai (cast `/Game/GGProjectExamples/Blueprints/Enemies/TestEnemy/TestEnemy_AI` (`AIBlueprintHelperLibrary.GetAIController` _loc_highestgradedai1)))
  (`/Game/GGProjectExamples/Blueprints/Enemies/TestEnemy/TestEnemy_AI.AIAttack` _astest_enemy_ai)
  (`BlueprintMapLibrary.Map_Add` (`self.EnemyGrading`) _loc_highestgradedai1 (`KismetMathLibrary.RandomFloatInRange` 1.0 5.0))
  (`self.UpdateWidget` _loc_highestgradedai1))

(fn `AddDebugWidgets`
  (params (EnemyInstance :type "/Game/GGProjectExamples/Blueprints/Enemies/TestEnemy/TestEnemy Object Reference"))
  (locals (Loc_Widget :type "/Game/GGProjectExamples/Blueprints/Enemies/DebugMeleeAI Object Reference"))
  (bind _enemygrading (`self.EnemyGrading`))
  (`BlueprintMapLibrary.Map_Add` _enemygrading EnemyInstance (`KismetMathLibrary.RandomFloatInRange` 1.0 5.0))
  (bind _returnvalue (`|CreateWidget` "/Game/GGProjectExamples/Blueprints/Enemies/DebugMeleeAI.DebugMeleeAI_C" null EnemyInstance (`BlueprintMapLibrary.Map_Find` _enemygrading EnemyInstance)))
  (bind _output_get (set `local.Loc_Widget` _returnvalue))
  (`BlueprintMapLibrary.Map_Add` (`self.EnemyWidgets`) EnemyInstance _output_get)
  (bind _returnvalue_2 (`AddComponent|NODE_AddWidgetComponent-0` :`self` EnemyInstance :`RelativeTransform` (`KismetMathLibrary.MakeTransform` (0.0 0.0 -100.0))))
  (`WidgetComponent.SetWidget` _returnvalue_2 _output_get))

(fn `FindHighestGrade`
  (returns (Loc_HighestValue1 :type "Float (double-precision)") (Loc_HighestGradedAI1 :type "/Game/GGProjectExamples/Blueprints/Enemies/TestEnemy/TestEnemy Object Reference"))
  (locals (Loc_HighestValue :type "Float (double-precision)") (Loc_HighestGradedAI :type "/Game/GGProjectExamples/Blueprints/Enemies/TestEnemy/TestEnemy Object Reference"))
  (bind _enemygrading (`self.EnemyGrading`))
  (bind _keys (`BlueprintMapLibrary.Map_Keys` _enemygrading))
  (for _array_element _keys
    (bind _value (`BlueprintMapLibrary.Map_Find` _enemygrading _array_element))
    (if (> _value (`local.Loc_HighestValue`))
      (set `local.Loc_HighestValue` _value)
      (bind _output_get (set `local.Loc_HighestGradedAI` _array_element))))
  (return (`local.Loc_HighestValue`) (`local.Loc_HighestGradedAI`)))

(fn `RecalculateGrades`
  (`self.ScoreByPosition`))

(fn `ScoreByPosition`
  (for _array_element (`self.EnemyList`)
    (`/Engine/EditorBlueprintResources/StandardMacros.IsValid` _array_element
      (:`Is Valid`
        (`BlueprintMapLibrary.Map_Add` (`self.EnemyGrading`) _array_element (+ (`KismetMathLibrary.NormalizeToRange` (* (`KismetMathLibrary.Dot_VectorVector` (`self.GetActorForwardVector` _array_element) (`self.GetActorForwardVector` (`GameplayStatics.GetPlayerCharacter` 0))) -1.0) -1.0 1.0) 0.5))))))

(fn `UpdateWidget`
  (params (EnemyInstance :type "/Game/GGProjectExamples/Blueprints/Enemies/TestEnemy/TestEnemy Object Reference"))
  (set `/Game/GGProjectExamples/Blueprints/Enemies/DebugMeleeAI.FightingGrade` (`BlueprintMapLibrary.Map_Find` (`self.EnemyGrading`) EnemyInstance) (`BlueprintMapLibrary.Map_Find` (`self.EnemyWidgets`) EnemyInstance)))

(fn `UserConstructionScript`)