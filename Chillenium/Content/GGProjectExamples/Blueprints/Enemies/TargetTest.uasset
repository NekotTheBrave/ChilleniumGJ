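; Test enemy that patrols waypoints, takes damage and shows its health on a health bar widget.
; AIMoveTo steps it along the Waypoints array, reversing at either end, with a random number of short navmesh roams after each waypoint reached.
; HitEnemy lowers health and updates the bar; at zero, it adds itself to the level save's DestroyedEnemies through the player character's game instance, then destroys itself.
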(event `FindNumberOfIndexes`
  (for (_ _array_index) (`self.Waypoints`)
    (set `self.NumberOfIndexes` _array_index)))

(event `self.ReceiveBeginPlay`
  (`self.MoveToNextWaypoint`)
  (bind _asaihealth_bar (cast `/Game/GGProjectExamples/Blueprints/Enemies/AIHealthBar` (`WidgetComponent.GetUserWidgetObject` (`self.HealthBar`))))
  (set `self.HealthWidgetRef` _asaihealth_bar)
  (set `/Game/GGProjectExamples/Blueprints/Enemies/AIHealthBar.MaxHealth` (`self.MaxHealth`) _asaihealth_bar))

(event `MoveToNextWaypoint`
  (if (>= (`self.CurrentIndex`) (`self.NumberOfIndexes`))
    (set `self.IsReverse` true)
    (elif (<= (`self.CurrentIndex`) 0)
      (set `self.IsReverse` false)))
  (if (`self.IsReverse`)
    (`|AIMoveTo` self (0.0 0.0 0.0) (`|GetArrayItem` (`self.Waypoints`) (`self.CurrentIndex`))
      (:`OnSuccess`
        (`KismetSystemLibrary.Delay` 0.2)
        (bind _result (`/Engine/EditorBlueprintResources/StandardMacros.DecrementInt` (`self.CurrentIndex`))
          (:`  `
            (set `self.CurrentIndex` _result)
            (`self.Roam`)))))
    (else
      (`|AIMoveTo` self (0.0 0.0 0.0) (`|GetArrayItem` (`self.Waypoints`) (`self.CurrentIndex`))
        (:`OnSuccess`
          (`KismetSystemLibrary.Delay` 0.2)
          (bind _result_2 (`/Engine/EditorBlueprintResources/StandardMacros.IncrementInt` (`self.CurrentIndex`))
            (:`  `
              (set `self.CurrentIndex` _result_2)
              (`self.Roam`))))))))

(event `Roam`
  (if (`self.IsRoamSet`)
    (if (>= (`self.CurrentRoam`) (`self.NumberOfRoam`))
      (set `self.IsRoamSet` false)
      (set `self.CurrentRoam` 0)
      (`self.MoveToNextWaypoint`)
      (else
        (`|AIMoveTo` self (`NavigationSystemV1.K2_GetRandomLocationInNavigableRadius` (`self.K2_GetActorLocation` self) 200.0 null null) null :!label _label
          (:`OnSuccess`
            (`KismetSystemLibrary.Delay` 2.0)
            (bind _result (`/Engine/EditorBlueprintResources/StandardMacros.IncrementInt` (`self.CurrentRoam`))
              (:`  `
                (set `self.CurrentRoam` _result)
                (`self.Roam`))))
          (:`OnFail`
            (`self.Roam`)))))
    (else
      (set `self.NumberOfRoam` (`KismetMathLibrary.RandomIntegerInRange` 1 5))
      (set `self.IsRoamSet` true)
      (goto _label))))

(event `/Game/GGProjectExamples/Blueprints/Enemies/TargettingInterface.HitEnemy`
  (params (Damage :type "Float (single-precision)"))
  (bind _output_get (set `self.Health` (- (`self.Health`) Damage)))
  (set `/Game/GGProjectExamples/Blueprints/Enemies/AIHealthBar.Health` _output_get (`self.HealthWidgetRef`))
  (if (<= _output_get 0.0)
    (bind _asgoth_girl_character (cast `/Game/GGProjectExamples/GothGirlCharacter/GothGirlCharacter` (`GameplayStatics.GetPlayerCharacter` 0)))
    (`KismetArrayLibrary.Array_AddUnique` (`/Game/GGProjectExamples/Blueprints/LevelDataObject.DestroyedEnemies` (`/Game/GGProjectExamples/Blueprints/GothGirlGameInstance.LevelSaveObject` (`/Game/GGProjectExamples/GothGirlCharacter/GothGirlCharacter.GothGirlGameInstance` _asgoth_girl_character))) self)
    (`self.K2_DestroyActor`)))

(fn `UserConstructionScript`)