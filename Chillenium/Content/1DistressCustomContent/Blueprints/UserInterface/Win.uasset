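; Win trigger actor that shows the victory screen when anything overlaps its Box component.
; The overlap adds a Win_Widget to the viewport, pauses the game, switches input to UI only and shows the mouse cursor.
; End opens MainMenuLevel only if the overlap's FromSweep value is true.
; Enter's level load sits on a branch that never runs and targets a level named "None".
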(event `self.Box.OnComponentBeginOverlap`
  (params (OverlappedComponent :type "PrimitiveComponent Object Reference") (OtherActor :type "Actor Object Reference") (OtherComp :type "PrimitiveComponent Object Reference") (OtherBodyIndex :type Integer) (bFromSweep :type Boolean) (SweepResult :type "HitResult Structure (by ref)"))
  (bind _returnvalue (`|CreateWidget` "/Game/1DistressCustomContent/Blueprints/UserInterface/Win_Widget.Win_Widget_C"))
  (`UserWidget.AddToViewport` _returnvalue 0)
  (`GameplayStatics.SetGamePaused` true)
  (`WidgetBlueprintLibrary.SetInputMode_UIOnlyEx` (`GameplayStatics.GetPlayerController` 0) null)
  (set `PlayerController.bShowMouseCursor` true (`GameplayStatics.GetPlayerController` 0)))

(event `Key|Enter`
  (params (Key :type "Key Structure"))
  (:`Pressed`
    (if (not true)
      (`GameplayStatics.OpenLevel` "None"))))

(event `Key|End`
  (params (Key :type "Key Structure"))
  (:`Pressed`
    (if (stale `self.Box.OnComponentBeginOverlap` bFromSweep)
      (`GameplayStatics.OpenLevel` "MainMenuLevel"))))

(fn `UserConstructionScript`)