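; Test enemy that patrols waypoints, chases the first-person player on sight, damages them on box overlap and dies to projectile hits.
; AIMoveTo drives a back-and-forth patrol with a few random navmesh wanders between waypoints.
; PawnSensing triggers the chase, with Tick switching sight radius by the visibility of the player's spotlight child component.
; A failed chase move returns it to patrol via a nearest-waypoint search.
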(event `FindNumberOfIndexes`
  (for (_ _array_index) (`self.Waypoints`)
    (set `self.NumberOfIndexes` _array_index)))

(event `self.Box.OnComponentBeginOverlap`
  (params (OverlappedComponent :type "PrimitiveComponent Object Reference") (OtherActor :type "Actor Object Reference") (OtherComp :type "PrimitiveComponent Object Reference") (OtherBodyIndex :type Integer) (bFromSweep :type Boolean) (SweepResult :type "HitResult Structure (by ref)"))
  (cast `/Game/1DistressCustomContent/Blueprints/Player/FirstPersonCharacter` (`GameplayStatics.GetPlayerCharacter` 0))
  (`GameplayStatics.ApplyDamage` (`GameplayStatics.GetPlayerCharacter` 0) (`self.Damage`))
  (`KismetSystemLibrary.PrintString` "-10 points")
  (`KismetSystemLibrary.Delay` 5.0))

(event `self.ReceiveBeginPlay`
  (`self.MoveToNextWaypoint`))

(event `MoveToNextWaypoint`
  (bind _shortestindex (`self.ShortestIndex`))
  (if (`self.WasBroken`)
    (set `self.WasBroken` false)
    (for (_array_element _array_index) (`self.Waypoints`)
      (bind _returnvalue (`self.GetDistanceTo` _array_element self))
      (`/Engine/EditorBlueprintResources/StandardMacros.CompareFloat` _returnvalue (`self.ShortestDistance`)
        (:`<`
          (set `self.ShortestDistance` _returnvalue)
          (set `self.ShortestIndex` _array_index))))
    (for (_array_element_2 _array_index_2) (`self.Waypoints`)
      (if (== _array_index_2 _shortestindex)
        (set `self.CurrentIndex` _shortestindex)
        (`|AIMoveTo` self (0.0 0.0 0.0) _array_element_2
          (:`then`
            (`KismetSystemLibrary.Delay` 2.0)
            (`self.MoveToNextWaypoint`)))))
    (else
      (if (>= (`self.CurrentIndex`) (`self.NumberOfIndexes`))
        (set `self.IsReverse` true)
        (elif (<= (`self.CurrentIndex`) 0)
          (set `self.IsReverse` false)))
      (if (`self.IsReverse`)
        (`|AIMoveTo` self (0.0 0.0 0.0) (`|GetArrayItem` (`self.Waypoints`) (`self.CurrentIndex`))
          (:`OnSuccess`
            (`KismetSystemLibrary.Delay` 1.0)
            (bind _result (`/Engine/EditorBlueprintResources/StandardMacros.DecrementInt` (`self.CurrentIndex`))
              (:`  `
                (set `self.CurrentIndex` _result)
                (`self.Roam`)))))
        (else
          (`|AIMoveTo` self (0.0 0.0 0.0) (`|GetArrayItem` (`self.Waypoints`) (`self.CurrentIndex`))
            (:`OnSuccess`
              (`KismetSystemLibrary.Delay` 1.0)
              (bind _result_2 (`/Engine/EditorBlueprintResources/StandardMacros.IncrementInt` (`self.CurrentIndex`))
                (:`  `
                  (set `self.CurrentIndex` _result_2)
                  (`self.Roam`))))))))))

(event `Roam`
  (if (`self.IsRoamSet`)
    (if (>= (`self.CurrentRoam`) (`self.NumberOfRoam`))
      (set `self.IsRoamSet` false)
      (set `self.CurrentRoam` 0)
      (`self.MoveToNextWaypoint`)
      (else
        (`|AIMoveTo` self (`NavigationSystemV1.K2_GetRandomLocationInNavigableRadius` (`self.K2_GetActorLocation` self) 200.0 null null) null :!label _label
          (:`OnSuccess`
            (`KismetSystemLibrary.Delay` 2.0)
            (bind _result (`/Engine/EditorBlueprintResources/StandardMacros.IncrementInt` (`self.CurrentRoam`))
              (:`  `
                (set `self.CurrentRoam` _result)
                (`self.Roam`))))
          (:`OnFail`
            (`self.Roam`)))))
    (else
      (set `self.NumberOfRoam` (`KismetMathLibrary.RandomIntegerInRange` 1 5))
      (set `self.IsRoamSet` true)
      (goto _label))))

(event `Chase`
  (if true
    (`|AIMoveTo` self (0.0 0.0 0.0) (`GameplayStatics.GetPlayerCharacter` 0) 1.0
      (:`OnSuccess`
        (`KismetSystemLibrary.Delay` 2.0)
        (`self.Chase`))
      (:`OnFail`
        (`KismetSystemLibrary.Delay` 2.0)
        (`self.MoveToNextWaypoint`)))))

(event `self.ReceiveTick`
  (params (DeltaSeconds :type "Float (single-precision)"))
  (bind _asfirst_person_character (cast `/Game/1DistressCustomContent/Blueprints/Player/FirstPersonCharacter` (`GameplayStatics.GetPlayerCharacter` 0)))
  (if (`SceneComponent.bVisible` (`SceneComponent.GetChildComponent` (`/Game/1DistressCustomContent/Blueprints/Player/FirstPersonCharacter.SpotLight` _asfirst_person_character) 0))
    (set `PawnSensingComponent.SightRadius` (`self.SightRadiusLight`) (`self.PawnSensing`))
    (else
      (set `PawnSensingComponent.SightRadius` (`self.SightRadiusDark`) (`self.PawnSensing`))))
  (add `PawnSensingComponent.OnSeePawn` (`self.PawnSensing`) (delegate `RoamToChase`)))

(event `RoamToChase`
  (params (Pawn :type "Pawn Object Reference"))
  (cast `/Game/1DistressCustomContent/Blueprints/Player/FirstPersonCharacter` Pawn)
  (set `self.WasBroken` true)
  (`self.Chase`))

(event `self.Cube.OnComponentBeginOverlap`
  (params (OverlappedComponent :type "PrimitiveComponent Object Reference") (OtherActor :type "Actor Object Reference") (OtherComp :type "PrimitiveComponent Object Reference") (OtherBodyIndex :type Integer) (bFromSweep :type Boolean) (SweepResult :type "HitResult Structure (by ref)"))
  (cast `/Game/1DistressCustomContent/Blueprints/Player/FirstPersonProjectile` OtherActor)
  (`self.K2_DestroyActor`))

(fn `UserConstructionScript`)