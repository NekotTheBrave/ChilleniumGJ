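; An interactable door that teleports whoever uses it to another place in the level.
; On Interact, it calls Teleport on the interacter, using the TeleportDestination actor's location and a rotation built from its own per-axis rotation variables.
; When a FirstPersonCharacter enters or leaves InteractRadius, the door's cube swaps between highlighted and normal materials.
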(event `/Game/1DistressCustomContent/Blueprints/InventorySystem/InteractInterface.Interact`
  (params (Interacter :type "Actor Object Reference"))
  (`self.K2_TeleportTo` Interacter (`self.K2_GetActorLocation` (`self.TeleportDestination`)) (`KismetMathLibrary.MakeRotator` (`self.TeleportRotationX`) (`self.TeleportRotationY`) (`self.TeleportRotationZ`))))

(event `self.InteractRadius.OnComponentBeginOverlap`
  (params (OverlappedComponent :type "PrimitiveComponent Object Reference") (OtherActor :type "Actor Object Reference") (OtherComp :type "PrimitiveComponent Object Reference") (OtherBodyIndex :type Integer) (bFromSweep :type Boolean) (SweepResult :type "HitResult Structure (by ref)"))
  (cast `/Game/1DistressCustomContent/Blueprints/Player/FirstPersonCharacter` OtherActor)
  (`PrimitiveComponent.SetMaterial` (`self.Cube`) 0 "/Game/1DistressCustomContent/Materials/Level1-1Materials/door3highlight.door3highlight"))

(event `self.InteractRadius.OnComponentEndOverlap`
  (params (OverlappedComponent :type "PrimitiveComponent Object Reference") (OtherActor :type "Actor Object Reference") (OtherComp :type "PrimitiveComponent Object Reference") (OtherBodyIndex :type Integer))
  (cast `/Game/1DistressCustomContent/Blueprints/Player/FirstPersonCharacter` OtherActor)
  (`PrimitiveComponent.SetMaterial` (`self.Cube`) 0 "/Game/1DistressCustomContent/Materials/Level1-1Materials/door3normal.door3normal"))

(fn `UserConstructionScript`)