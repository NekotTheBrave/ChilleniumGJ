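; Medkit pickup item that restores the first-person player's health when used.
; Overlapping its ItemRadius with the player character swaps both base mesh materials, and leaving swaps in a second pair, signalling proximity.
; UseItem runs the parent item logic, then adds a fixed amount to player 0's CurrentHealth, clamped to MaxHealth, and returns the parent's result.
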(event `self.ItemRadius.OnComponentBeginOverlap`
  (params (OverlappedComponent :type "PrimitiveComponent Object Reference") (OtherActor :type "Actor Object Reference") (OtherComp :type "PrimitiveComponent Object Reference") (OtherBodyIndex :type Integer) (bFromSweep :type Boolean) (SweepResult :type "HitResult Structure (by ref)"))
  (bind _basemesh (`self.BaseMesh`))
  (cast `/Game/1DistressCustomContent/Blueprints/Player/FirstPersonCharacter` OtherActor)
  (`PrimitiveComponent.SetMaterial` _basemesh 0 "/Game/1DistressCustomContent/Materials/NickelInstance.NickelInstance")
  (`PrimitiveComponent.SetMaterial` _basemesh 1 "/Game/1DistressCustomContent/Materials/BasicFloorTest.BasicFloorTest"))

(event `self.ItemRadius.OnComponentEndOverlap`
  (params (OverlappedComponent :type "PrimitiveComponent Object Reference") (OtherActor :type "Actor Object Reference") (OtherComp :type "PrimitiveComponent Object Reference") (OtherBodyIndex :type Integer))
  (bind _basemesh (`self.BaseMesh`))
  (cast `/Game/1DistressCustomContent/Blueprints/Player/FirstPersonCharacter` OtherActor)
  (`PrimitiveComponent.SetMaterial` _basemesh 0 "/Game/1DistressCustomContent/Materials/NickelInstance1.NickelInstance1")
  (`PrimitiveComponent.SetMaterial` _basemesh 1 "/Game/1DistressCustomContent/Materials/BasicFloorTest1.BasicFloorTest1"))

(fn `UseItem`
  (returns (Success :type Boolean))
  (bind _success (`parent.UseItem`))
  (bind _asfirst_person_character (cast `/Game/1DistressCustomContent/Blueprints/Player/FirstPersonCharacter` (`GameplayStatics.GetPlayerCharacter` 0)))
  (set `/Game/1DistressCustomContent/Blueprints/Player/FirstPersonCharacter.CurrentHealth` (`KismetMathLibrary.FClamp` (+ (`/Game/1DistressCustomContent/Blueprints/Player/FirstPersonCharacter.CurrentHealth` _asfirst_person_character) 25.0) 0.0 (`/Game/1DistressCustomContent/Blueprints/Player/FirstPersonCharacter.MaxHealth` _asfirst_person_character)) _asfirst_person_character)
  (return _success))

(fn `UserConstructionScript`)