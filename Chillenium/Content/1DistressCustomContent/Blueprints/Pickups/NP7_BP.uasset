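; NP7_BP is an interactable news clipping pickup that opens a UI view when used.
; Interact creates NP7_Widget, adds it to the viewport, pauses the game and switches to UI-only input with the mouse cursor shown.
; ItemRadius overlaps with FirstPersonCharacter set the Cube's highlight material.
; Begin and end overlap both apply the same News_clipping_7Highlight1 material, so leaving the radius does not clear the highlight.
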(event `/Game/1DistressCustomContent/Blueprints/InventorySystem/InteractInterface.Interact`
  (params (Interacter :type "Actor Object Reference"))
  (bind _returnvalue (`GameplayStatics.GetPlayerController` 0))
  (bind _returnvalue_2 (`|CreateWidget` "/Game/1DistressCustomContent/Blueprints/UserInterface/NP7_Widget.NP7_Widget_C" (`GameplayStatics.GetPlayerController` 0)))
  (`UserWidget.AddToViewport` _returnvalue_2 0)
  (`GameplayStatics.SetGamePaused` true)
  (`WidgetBlueprintLibrary.SetInputMode_UIOnlyEx` _returnvalue _returnvalue_2 "LockAlways")
  (set `PlayerController.bShowMouseCursor` true _returnvalue))

(event `self.ItemRadius.OnComponentBeginOverlap`
  (params (OverlappedComponent :type "PrimitiveComponent Object Reference") (OtherActor :type "Actor Object Reference") (OtherComp :type "PrimitiveComponent Object Reference") (OtherBodyIndex :type Integer) (bFromSweep :type Boolean) (SweepResult :type "HitResult Structure (by ref)"))
  (cast `/Game/1DistressCustomContent/Blueprints/Player/FirstPersonCharacter` OtherActor)
  (`PrimitiveComponent.SetMaterial` (`self.Cube`) 0 "/Game/1DistressCustomContent/Materials/Level1-1Materials/News_clipping_7Highlight1.News_clipping_7Highlight1"))

(event `self.ItemRadius.OnComponentEndOverlap`
  (params (OverlappedComponent :type "PrimitiveComponent Object Reference") (OtherActor :type "Actor Object Reference") (OtherComp :type "PrimitiveComponent Object Reference") (OtherBodyIndex :type Integer))
  (cast `/Game/1DistressCustomContent/Blueprints/Player/FirstPersonCharacter` OtherActor)
  (`PrimitiveComponent.SetMaterial` (`self.Cube`) 0 "/Game/1DistressCustomContent/Materials/Level1-1Materials/News_clipping_7Highlight1.News_clipping_7Highlight1"))

(fn `UserConstructionScript`)